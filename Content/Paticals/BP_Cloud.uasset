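; BP_Cloud is a short-lived cloud effect built on a Sphere component that fades in, grows, fades out and destroys itself.
; Tick raises opacity to about 0.9, then scales the sphere up toward Size until BeginPlay's timed Fade flag switches it to fading out.
; Steps are fixed per frame, so speed follows frame rate, and each opacity step creates a new dynamic material instance.
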(event `self.ReceiveBeginPlay`
  (`KismetSystemLibrary.Delay` 3.5)
  (set `self.Fade` true)
  (`KismetSystemLibrary.Delay` 4.0)
  (`self.K2_DestroyActor`))

(event `self.ReceiveTick`
  (params (DeltaSeconds :type "Float (single-precision)"))
  (bind _returnvalue (- (`self.opacity`) 0.01))
  (bind (_returnvalue_x _returnvalue_y _returnvalue_z) (`KismetMathLibrary.BreakVector` (`SceneComponent.K2_GetComponentScale` (`self.Sphere`))))
  (bind _returnvalue_2 (+ (`self.opacity`) 0.03))
  (if (`self.Fade`)
    (bind _returnvalue_3 (`PrimitiveComponent.CreateDynamicMaterialInstance` (`self.Sphere`) 0 "/Game/Materials/InstMats/Cloud.Cloud" "None"))
    (`MaterialInstanceDynamic.SetScalarParameterValue` _returnvalue_3 "Opacity" _returnvalue)
    (set `self.opacity` _returnvalue)
    (elif (< (`self.opacity`) 0.9)
      (bind _returnvalue_4 (`PrimitiveComponent.CreateDynamicMaterialInstance` (`self.Sphere`) 0 "/Game/Materials/InstMats/Cloud.Cloud" "None"))
      (`MaterialInstanceDynamic.SetScalarParameterValue` _returnvalue_4 "Opacity" _returnvalue_2)
      (set `self.opacity` _returnvalue_2)
      (elif (< _returnvalue_x (`self.Size`))
        (`SceneComponent.SetWorldScale3D` (`self.Sphere`) (`KismetMathLibrary.MakeVector` (+ _returnvalue_x 0.05) (+ _returnvalue_y 0.05) (+ _returnvalue_z 0.05)))))))

(fn `UserConstructionScript`)