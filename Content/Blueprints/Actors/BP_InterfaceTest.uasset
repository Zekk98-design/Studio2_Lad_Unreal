(event `/Game/Blueprints/Interface/I_InteractivePlot.SelectOff`
  (params (Name :type String))
  (if (`KismetStringLibrary.EqualEqual_StrStr` Name (`KismetSystemLibrary.GetObjectName` self))
    (set `self.Selected` false)))

(event `/Game/Blueprints/Interface/I_InteractivePlot.SelectOn`
  (params (Name :type String))
  (if (`KismetStringLibrary.EqualEqual_StrStr` Name (`KismetSystemLibrary.GetObjectName` self))
    (set `self.Selected` true)))

(event `/Game/Blueprints/Interface/I_InteractivePlot.HoverOn`
  (params (Name :type String))
  (if (`KismetStringLibrary.EqualEqual_StrStr` Name (`KismetSystemLibrary.GetObjectName` self))
    (set `self.Hovered` true)
    (set `self.CurrentSelectionCounter` (`self.SelectionCounter`))))

(event `/Game/Blueprints/Interface/I_InteractivePlot.IBuild`
  (params (IBuildingType :type Name) (IBuildingID :type Integer) (Name :type String))
  (if (`KismetStringLibrary.EqualEqual_StrStr` Name (`KismetSystemLibrary.GetObjectName` self))
    (`self.Build` IBuildingType IBuildingID)))

(event `self.ReceiveBeginPlay`
  (`SceneComponent.SetVisibility` (`self.SelectedBox`) (`self.Hovered`) true))

(event `self.ReceiveTick`
  (params (DeltaSeconds :type "Float (single-precision)"))
  (bind _returnvalue (or (`self.Hovered`) (`self.Selected`)))
  (if (!= _returnvalue (`SceneComponent.IsVisible` (`self.SelectedBox`)))
    (`SceneComponent.SetVisibility` (`self.SelectedBox`) _returnvalue true))
  (if (and (`self.Hovered`) (> (`self.CurrentSelectionCounter`) 0.0))
    (set `self.CurrentSelectionCounter` (- (`self.CurrentSelectionCounter`) (`GameplayStatics.GetWorldDeltaSeconds`)))
    (elif (not (`self.Selected`))
      (set `self.Hovered` false))))

(fn `Build`
  (params (BuildingType :type Name) (BuildingID :type Integer))
  (locals (LocBuildingType :type Name) (LocBuildingID :type Integer))
  (set `local.LocBuildingID` BuildingID)
  (switch `name` BuildingType
    (:`Housing`
      ;[1 1 1] Housing
      (`|SpawnActorFromClass` (`|GetArrayItem` (`self.Houses`) (`local.LocBuildingID`)) (`SceneComponent.K2_GetComponentToWorld` (`self.DefaultSceneRoot`)) "Undefined" "OverrideRootScale" null null)
      (`self.K2_DestroyActor`))
    (:`Storage`
      ;[1 1 1] Storage
      (`|SpawnActorFromClass` (`|GetArrayItem` (`self.Storage`) (`local.LocBuildingID`)) (`SceneComponent.K2_GetComponentToWorld` (`self.DefaultSceneRoot`)) "Undefined" "OverrideRootScale" null null)
      (`self.K2_DestroyActor`))
    (:`Services`
      ;[1 1 1] Services
      (`|SpawnActorFromClass` (`|GetArrayItem` (`self.Services`) (`local.LocBuildingID`)) (`SceneComponent.K2_GetComponentToWorld` (`self.DefaultSceneRoot`)) "Undefined" "OverrideRootScale" null null)
      (`self.K2_DestroyActor`))
    (:`Defence`
      ;[1 1 1] Defence
      (`|SpawnActorFromClass` (`|GetArrayItem` (`self.Defence`) (`local.LocBuildingID`)) (`SceneComponent.K2_GetComponentToWorld` (`self.DefaultSceneRoot`)) "Undefined" "OverrideRootScale" null null)
      (`self.K2_DestroyActor`))))

(fn `UserConstructionScript`)