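; BP_Rocket is an actor whose Rocket component climbs straight up in world space.
; Each Tick adds Speed to the component's Z location, then grows Speed by a small multiplier while it is below MaxSpeed, giving an exponential acceleration up to a cap.
; Movement and acceleration ignore delta time, so both depend on frame rate.
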(event `self.ReceiveTick`
  (params (DeltaSeconds :type "Float (single-precision)"))
  (bind _rocket (`self.Rocket`))
  (bind (_returnvalue_x _returnvalue_y _returnvalue_z) (`KismetMathLibrary.BreakVector` (`SceneComponent.K2_GetComponentLocation` _rocket)))
  (`SceneComponent.K2_SetWorldLocation` _rocket (`KismetMathLibrary.MakeVector` _returnvalue_x _returnvalue_y (+ _returnvalue_z (`self.Speed`))) false false)
  (if (< (`self.Speed`) (`self.MaxSpeed`))
    (set `self.Speed` (* (`self.Speed`) 1.005))))

(fn `UserConstructionScript`)