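; BP_InteractivePen is a pen pickup actor that can be grabbed, released and outlined.
; Pickup toggles Capsule physics and attaches the root to the given hand or detaches it, keeping world transform.
; SetHighlight enables custom depth with a stencil value on Cube and Cone and arms a short countdown.
; Tick's countdown subtraction is reversed, so an unrefreshed highlight clears by the second tick instead of timing out.
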(event `self.ReceiveBeginPlay`)

(event `self.ReceiveTick`
  (params (DeltaSeconds :type "Float (single-precision)"))
  (bind _cube (`self.Cube`))
  (bind _returnvalue (- DeltaSeconds (`self.HighlightCountdown`)))
  (if (< _returnvalue 0.0)
    (set `self.HighlightCountdown` _returnvalue)
    (else
      (`PrimitiveComponent.SetRenderCustomDepth` _cube false)
      (`PrimitiveComponent.SetRenderCustomDepth` (`self.Cone`) false)
      (`PrimitiveComponent.SetCustomDepthStencilValue` _cube 0)
      (`PrimitiveComponent.SetCustomDepthStencilValue` (`self.Cone`) 0))))

(event `/Game/Blueprints/Interface/I_Pickupable.Pickup`
  (params (Hand :type "SceneComponent Object Reference") (bHolding :type Boolean))
  (bind _capsule (`self.Capsule`))
  (if bHolding
    (`PrimitiveComponent.SetSimulatePhysics` _capsule false)
    (`SceneComponent.K2_AttachToComponent` (`self.K2_GetRootComponent`) Hand "None" "KeepWorld" "KeepWorld" "KeepWorld" false)
    (else
      (`PrimitiveComponent.SetSimulatePhysics` _capsule true)
      (`self.K2_DetachFromActor` "KeepWorld" "KeepWorld" "KeepWorld"))))

(event `/Game/Blueprints/Interface/I_Pickupable.SetHighlight`
  (params (Highlight :type Boolean))
  (bind _cube (`self.Cube`))
  (`PrimitiveComponent.SetRenderCustomDepth` _cube true)
  (`PrimitiveComponent.SetRenderCustomDepth` (`self.Cone`) true)
  (`PrimitiveComponent.SetCustomDepthStencilValue` _cube 2)
  (`PrimitiveComponent.SetCustomDepthStencilValue` (`self.Cone`) 2)
  (set `self.HighlightCountdown` 0.1))

(fn `UserConstructionScript`)