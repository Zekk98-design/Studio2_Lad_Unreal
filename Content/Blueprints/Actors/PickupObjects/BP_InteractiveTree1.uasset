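; Pickup tree actor, apparently for VR, whose foliage reflects the game's environment state.
; Pickup attaches it to the hand with physics off, or detaches it and restores physics.
; SetHighlight enables a custom-depth stencil outline and sets a countdown that Tick checks to clear it.
; That same Tick branch, after a random delay, reads VRGameMode's EnvironmentState to swap leaf materials, hiding leaves when Dead.
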(event `/Game/Blueprints/Interface/I_Pickupable.Pickup`
  (params (Hand :type "SceneComponent Object Reference") (bHolding :type Boolean))
  (bind _tree (`self.Tree`))
  (if bHolding
    (`PrimitiveComponent.SetSimulatePhysics` _tree false)
    (`SceneComponent.K2_AttachToComponent` (`self.K2_GetRootComponent`) Hand "None" "KeepWorld" "KeepWorld" "KeepWorld" false)
    (else
      (`PrimitiveComponent.SetSimulatePhysics` _tree true)
      (`self.K2_DetachFromActor` "KeepWorld" "KeepWorld" "KeepWorld"))))

(event `self.ReceiveBeginPlay`
  (bind _asvrgame_mode (cast `/Game/Blueprints/VRGameMode` (`GameplayStatics.GetGameMode`)))
  (set `self.Gamemode` _asvrgame_mode))

(event `self.ReceiveTick`
  (params (DeltaSeconds :type "Float (single-precision)"))
  (bind _tree (`self.Tree`))
  (bind _leaves (`self.Leaves`))
  (bind _returnvalue (- DeltaSeconds (`self.HighlightCountdown`)))
  (bind _environmentstate (`/Game/Blueprints/VRGameMode.EnvironmentState` (`self.Gamemode`)))
  (bind _output (`|GetArrayItem` (`self.Materials`) (`KismetMathLibrary.Conv_ByteToInt` _environmentstate)))
  (if (< _returnvalue 0.0)
    (set `self.HighlightCountdown` _returnvalue)
    (else
      (`PrimitiveComponent.SetRenderCustomDepth` _tree false)
      (`PrimitiveComponent.SetCustomDepthStencilValue` _tree 0)
      (`KismetSystemLibrary.Delay` (`KismetMathLibrary.RandomFloatInRange` 2.0 12.0))
      (`SceneComponent.SetVisibility` (`self.Leaves`) true false)
      (`SceneComponent.SetVisibility` (`self.Leaves1`) true false)
      (switch `/Game/Blueprints/Enum_TreeState` _environmentstate
        (:`NewEnumerator0`
          (`PrimitiveComponent.SetMaterial` _leaves 0 _output)
          (`PrimitiveComponent.SetMaterial` (`self.Leaves1`) 0 _output))
        (:`NewEnumerator1`
          (`PrimitiveComponent.SetMaterial` _leaves 0 _output)
          (`PrimitiveComponent.SetMaterial` (`self.Leaves1`) 0 _output))
        (:`NewEnumerator2`
          (`PrimitiveComponent.SetMaterial` _leaves 0 _output)
          (`PrimitiveComponent.SetMaterial` (`self.Leaves1`) 0 _output))
        (:`NewEnumerator3`
          (`SceneComponent.SetVisibility` _leaves false false)
          (`SceneComponent.SetVisibility` (`self.Leaves1`) false false))))))

(event `/Game/Blueprints/Interface/I_Pickupable.SetHighlight`
  (params (Highlight :type Boolean))
  (bind _tree (`self.Tree`))
  (`PrimitiveComponent.SetRenderCustomDepth` _tree Highlight)
  (`PrimitiveComponent.SetCustomDepthStencilValue` _tree 2)
  (set `self.HighlightCountdown` 0.1))

(fn `UserConstructionScript`)