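; BP_NuclearWaste is a physics-simulated nuclear waste object that can be picked up and released in a VR game.
; Its Pickup event either stops physics and attaches the root component to the given Hand, or restores physics and detaches, keeping world transform.
; BeginPlay caches the VRGameMode, and GetUnstoredWaste adds this object's WasteCarried to that game mode's UnstoredWaste total.
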(event `/Game/Blueprints/Interface/I_NuclearWaste.GetUnstoredWaste`
  (bind _vrgamemode (`self.VRGameMode`))
  (set `/Game/Blueprints/VRGameMode.UnstoredWaste` (+ (`/Game/Blueprints/VRGameMode.UnstoredWaste` _vrgamemode) (`self.WasteCarried`)) _vrgamemode))

(event `self.ReceiveBeginPlay`
  (`PrimitiveComponent.SetSimulatePhysics` (`self.StaticMesh`) true)
  (bind _asvrgame_mode (cast `/Game/Blueprints/VRGameMode` (`GameplayStatics.GetGameMode`)))
  (set `self.VRGameMode` _asvrgame_mode))

(event `self.ReceiveTick`
  (params (DeltaSeconds :type "Float (single-precision)")))

(event `/Game/Blueprints/Interface/I_Pickupable.Pickup`
  (params (Hand :type "SceneComponent Object Reference") (bHolding :type Boolean))
  (if bHolding
    (`PrimitiveComponent.SetSimulatePhysics` (`self.StaticMesh`) false)
    (`SceneComponent.K2_AttachToComponent` (`self.K2_GetRootComponent`) Hand "None" "KeepWorld" "KeepWorld" "KeepWorld" false)
    (else
      (`PrimitiveComponent.SetSimulatePhysics` (`self.StaticMesh`) true)
      (`self.K2_DetachFromActor` "KeepWorld" "KeepWorld" "KeepWorld"))))

(fn `UserConstructionScript`)