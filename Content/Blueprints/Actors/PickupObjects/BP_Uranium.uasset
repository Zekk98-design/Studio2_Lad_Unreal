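; Uranium pickup actor whose physics-simulated mesh can be held in a hand and highlighted.
; Pickup disables physics and attaches the root to the hand, then restores physics and detaches on release.
; SetHighlight drives custom depth and stencil and arms a short countdown.
; Tick clears the highlight unless refreshed, though its reversed subtraction turns the countdown negative, so it expires within about two frames.
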(event `self.ReceiveBeginPlay`
  (`PrimitiveComponent.SetSimulatePhysics` (`self.StaticMesh`) true))

(event `self.ReceiveTick`
  (params (DeltaSeconds :type "Float (single-precision)"))
  (bind _staticmesh (`self.StaticMesh`))
  (bind _returnvalue (- DeltaSeconds (`self.HighlightCountdown`)))
  (if (< _returnvalue 0.0)
    (set `self.HighlightCountdown` _returnvalue)
    (else
      (`PrimitiveComponent.SetRenderCustomDepth` _staticmesh false)
      (`PrimitiveComponent.SetCustomDepthStencilValue` _staticmesh 0))))

(event `/Game/Blueprints/Interface/I_Pickupable.Pickup`
  (params (Hand :type "SceneComponent Object Reference") (bHolding :type Boolean))
  (if bHolding
    (`PrimitiveComponent.SetSimulatePhysics` (`self.StaticMesh`) false)
    (`SceneComponent.K2_AttachToComponent` (`self.K2_GetRootComponent`) Hand "None" "KeepWorld" "KeepWorld" "KeepWorld" false)
    (else
      (`PrimitiveComponent.SetSimulatePhysics` (`self.StaticMesh`) true)
      (`self.K2_DetachFromActor` "KeepWorld" "KeepWorld" "KeepWorld"))))

(event `/Game/Blueprints/Interface/I_Pickupable.SetHighlight`
  (params (Highlight :type Boolean))
  (bind _staticmesh (`self.StaticMesh`))
  (`PrimitiveComponent.SetRenderCustomDepth` _staticmesh Highlight)
  (`PrimitiveComponent.SetCustomDepthStencilValue` _staticmesh 2)
  (set `self.HighlightCountdown` 0.1))

(fn `UserConstructionScript`)