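; Entertainment building actor for a VR game that can be selected, upgraded through four visual levels or demolished into an empty plot.
; Name-matched events drive selection, upgrade and demolition; Tick shows the selection box while selected or hovered, with hover expiring on a countdown.
; Upgrades toggle level root visibility.
; BeginPlay, upgrade and demolish keep VRGameMode's AllBuildings list updated using "Entertainment" plus level as the entry name.
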(event `/Game/Blueprints/Interface/I_InteractivePlot.SelectOff`
  (params (Name :type String))
  ;[1 1 1] Selecting & player feedback
  (if (`KismetStringLibrary.EqualEqual_StrStr` Name (`KismetSystemLibrary.GetObjectName` self))
    (set `self.Selected` false)))

(event `/Game/Blueprints/Interface/I_InteractivePlot.SelectOn`
  (params (Name :type String))
  ;[1 1 1] Selecting & player feedback
  (if (`KismetStringLibrary.EqualEqual_StrStr` Name (`KismetSystemLibrary.GetObjectName` self))
    (set `self.Selected` true)))

(event `/Game/Blueprints/Interface/I_InteractivePlot.HoverOn`
  (params (Name :type String))
  ;[1 1 1] Selecting & player feedback
  (if (`KismetStringLibrary.EqualEqual_StrStr` Name (`KismetSystemLibrary.GetObjectName` self))
    (set `self.Hovered` true)
    (set `self.CurrentSelectionCounter` (`self.SelectionCounter`))))

(event `/Game/Blueprints/Interface/I_Demolishable.IDemolish`
  (params (IName :type String))
  ;[1 1 1] Destory building
  (if (`KismetStringLibrary.EqualEqual_StrStr` IName (`KismetSystemLibrary.GetObjectName` self))
    (`self.Demolish`)))

(event `self.ReceiveBeginPlay`
  ;[1 1 1] Begin Play
  (`SceneComponent.SetVisibility` (`self.SelectedBox`) (`self.Hovered`) true)
  ;[1 1 1] Set upgrade array
  (`KismetArrayLibrary.Array_Add` (`self.UpgradeLevelsRoots`) (`self.UpgradeLevel0`))
  (`KismetArrayLibrary.Array_Add` (`self.UpgradeLevelsRoots`) (`self.UpgradeLevel1`))
  (`KismetArrayLibrary.Array_Add` (`self.UpgradeLevelsRoots`) (`self.UpgradeLevel2`))
  (`KismetArrayLibrary.Array_Add` (`self.UpgradeLevelsRoots`) (`self.UpgradeLevel3`))
  (`self.SetVisibility`)
  (bind _asvrgame_mode (cast `/Game/Blueprints/VRGameMode` (`GameplayStatics.GetGameMode`)))
  (bind _output_get (set `self.VRGameMode` _asvrgame_mode))
  (`KismetArrayLibrary.Array_Add` (`/Game/Blueprints/VRGameMode.AllBuildings` _output_get) (`KismetStringLibrary.Conv_StringToName` (`KismetStringLibrary.Concat_StrStr` "Entertainment" (`KismetStringLibrary.Conv_IntToString` (`self.CurrentLevel`))))))

(event `/Game/Blueprints/Interface/I_UpgradeAble.IUpgrade`
  (params (Name :type String))
  (if (`KismetStringLibrary.EqualEqual_StrStr` Name (`KismetSystemLibrary.GetObjectName` self))
    (`self.Upgrade`)))

(event `self.ReceiveTick`
  (params (DeltaSeconds :type "Float (single-precision)"))
  (bind _returnvalue (or (`self.Hovered`) (`self.Selected`)))
  ;[1 1 1] Tick
  (if (!= _returnvalue (`SceneComponent.IsVisible` (`self.SelectedBox`)))
    (`SceneComponent.SetVisibility` (`self.SelectedBox`) _returnvalue true))
  (if (and (`self.Hovered`) (> (`self.CurrentSelectionCounter`) 0.0))
    (set `self.CurrentSelectionCounter` (- (`self.CurrentSelectionCounter`) (`GameplayStatics.GetWorldDeltaSeconds`)))
    (elif (not (`self.Selected`))
      (set `self.Hovered` false))))

(fn `Demolish`
  (locals (Deleted :type Boolean))
  (for (_array_element _array_index) (`/Game/Blueprints/VRGameMode.AllBuildings` (`self.VRGameMode`))
    (if (and (not (`local.Deleted`)) (== _array_element (`KismetStringLibrary.Conv_StringToName` (`KismetStringLibrary.Concat_StrStr` "Entertainment" (`KismetStringLibrary.Conv_IntToString` (`self.CurrentLevel`))))))
      (`KismetArrayLibrary.Array_Remove` (`/Game/Blueprints/VRGameMode.AllBuildings` (`self.VRGameMode`)) _array_index)
      (set `local.Deleted` false)))
  (`|SpawnActorFromClass` "/Game/Blueprints/Actors/MainBuildings/BP_EmptyPlot.BP_EmptyPlot_C" (`SceneComponent.K2_GetComponentToWorld` (`self.DefaultSceneRoot`)) "Undefined" "OverrideRootScale" null null)
  (`self.K2_DestroyActor`))

(fn `SetVisibility`
  (locals (LocBuildingID :type Integer))
  (for (_ _array_index) (`self.UpgradeLevelsRoots`)
    (`SceneComponent.SetVisibility` (`|GetArrayItem` (`self.UpgradeLevelsRoots`) _array_index) (== _array_index (`self.CurrentLevel`)) true)))

(fn `Upgrade`
  (locals (Deleted :type Boolean))
  (bind _allbuildings (`/Game/Blueprints/VRGameMode.AllBuildings` (`self.VRGameMode`)))
  (if (< (+ (`self.CurrentLevel`) 1) (`KismetArrayLibrary.Array_Length` (`self.UpgradeLevelsRoots`)))
    (`/Engine/EditorBlueprintResources/StandardMacros.IncrementInt` (`self.CurrentLevel`)
      (:`  `
        (`self.SetVisibility`)
        (for (_array_element _array_index) _allbuildings
          (if (and (not (`local.Deleted`)) (== _array_element (`KismetStringLibrary.Conv_StringToName` (`KismetStringLibrary.Concat_StrStr` "Entertainment" (`KismetStringLibrary.Conv_IntToString` (- (`self.CurrentLevel`) 1))))))
            (`KismetArrayLibrary.Array_Remove` (`/Game/Blueprints/VRGameMode.AllBuildings` (`self.VRGameMode`)) _array_index)
            (set `local.Deleted` true)))
        (`KismetArrayLibrary.Array_Add` _allbuildings (`KismetStringLibrary.Conv_StringToName` (`KismetStringLibrary.Concat_StrStr` "Entertainment" (`KismetStringLibrary.Conv_IntToString` (`self.CurrentLevel`)))))))))

(fn `UserConstructionScript`)