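; Storage building actor that can be hovered, selected, upgraded or demolished.
; Events act only when the passed name matches this actor's object name.
; Tick shows the selection box while hovered or selected, letting hover expire through a countdown that each hover event refreshes.
; Upgrade spawns the class after its own in the Storage array and Demolish spawns an empty plot, each at the same transform before destroying this actor.
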(event `/Game/Blueprints/Interface/I_InteractivePlot.SelectOff`
  (params (Name :type String))
  (if (`KismetStringLibrary.EqualEqual_StrStr` Name (`KismetSystemLibrary.GetObjectName` self))
    (set `self.Selected` false)))

(event `/Game/Blueprints/Interface/I_InteractivePlot.SelectOn`
  (params (Name :type String))
  (if (`KismetStringLibrary.EqualEqual_StrStr` Name (`KismetSystemLibrary.GetObjectName` self))
    (set `self.Selected` true)))

(event `/Game/Blueprints/Interface/I_InteractivePlot.HoverOn`
  (params (Name :type String))
  (if (`KismetStringLibrary.EqualEqual_StrStr` Name (`KismetSystemLibrary.GetObjectName` self))
    (set `self.Hovered` true)
    (set `self.CurrentSelectionCounter` (`self.SelectionCounter`))))

(event `/Game/Blueprints/Interface/I_Housing+StoragePlot.IDemolish`
  (params (Name :type String))
  (if (`KismetStringLibrary.EqualEqual_StrStr` Name (`KismetSystemLibrary.GetObjectName` self))
    (`self.Demolish`)
    (`KismetSystemLibrary.PrintString` "Demolished")))

(event `self.ReceiveBeginPlay`
  (`SceneComponent.SetVisibility` (`self.SelectedBox`) (`self.Hovered`) true))

(event `/Game/Blueprints/Interface/I_Housing+StoragePlot.IUpgrade`
  (params (Name :type String))
  (if (`KismetStringLibrary.EqualEqual_StrStr` Name (`KismetSystemLibrary.GetObjectName` self))
    (`self.Upgrade`)))

(event `self.ReceiveTick`
  (params (DeltaSeconds :type "Float (single-precision)"))
  (bind _returnvalue (or (`self.Hovered`) (`self.Selected`)))
  (if (!= _returnvalue (`SceneComponent.IsVisible` (`self.SelectedBox`)))
    (`SceneComponent.SetVisibility` (`self.SelectedBox`) _returnvalue true))
  (if (and (`self.Hovered`) (> (`self.CurrentSelectionCounter`) 0.0))
    (set `self.CurrentSelectionCounter` (- (`self.CurrentSelectionCounter`) (`GameplayStatics.GetWorldDeltaSeconds`)))
    (elif (not (`self.Selected`))
      (set `self.Hovered` false))))

(fn `Demolish`
  (`|SpawnActorFromClass` "/Game/Blueprints/Actors/MainBuildings/BP_EmptyPlotInterface.BP_EmptyPlotInterface_C" (`SceneComponent.K2_GetComponentToWorld` (`self.DefaultSceneRoot`)) "Undefined" "OverrideRootScale" null null)
  (`self.K2_DestroyActor`))

(fn `Upgrade`
  (locals (LocBuildingID :type Integer))
  (bind _returnvalue (+ (`local.LocBuildingID`) 1))
  (for (_array_element _array_index) (`self.Storage`)
    (if (== _array_element (`GameplayStatics.GetObjectClass` self))
      (set `local.LocBuildingID` _array_index)))
  (if (<= _returnvalue (`KismetArrayLibrary.Array_Length` (`self.Storage`)))
    (`|SpawnActorFromClass` (`|GetArrayItem` (`self.Storage`) _returnvalue) (`SceneComponent.K2_GetComponentToWorld` (`self.DefaultSceneRoot`)) "Undefined" "OverrideRootScale" null null)
    (`self.K2_DestroyActor`)))

(fn `UserConstructionScript`)