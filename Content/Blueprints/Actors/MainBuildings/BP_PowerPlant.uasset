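; BP_PowerPlant is an upgradeable power plant building that adjusts the VR game mode's current power.
; Its events act only when the passed name matches the actor; power changes step by 10 but clamp to 0–1, snapping to either limit.
; Tick shows the selection box while hovered or selected, expiring hover through a countdown refreshed by Hoveron.
; Upgrades advance the level and show only that level's root component.
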(event `/Game/Blueprints/Interface/I_PowerPlant.IncreasePower`
  (params (Name :type String))
  (bind _vrgamemode (`self.VRGameMode`))
  (if (`KismetStringLibrary.EqualEqual_StrStr` Name (`KismetSystemLibrary.GetObjectName` self))
    (bind _output_get (set `/Game/Blueprints/VRGameMode.CurrentPower` (`KismetMathLibrary.FClamp` (+ (`/Game/Blueprints/VRGameMode.CurrentPower` _vrgamemode) 10.0)) _vrgamemode))
    (`KismetSystemLibrary.PrintString` (`KismetStringLibrary.Conv_DoubleToString` (stale `/Game/Blueprints/Interface/I_PowerPlant.DecreasePower` _output_get)) :!label _label)))

(event `/Game/Blueprints/Interface/I_PowerPlant.DecreasePower`
  (params (Name :type String))
  (bind _vrgamemode (`self.VRGameMode`))
  (if (`KismetStringLibrary.EqualEqual_StrStr` Name (`KismetSystemLibrary.GetObjectName` self))
    (bind _output_get (set `/Game/Blueprints/VRGameMode.CurrentPower` (`KismetMathLibrary.FClamp` (- (`/Game/Blueprints/VRGameMode.CurrentPower` _vrgamemode) 10.0)) _vrgamemode))
    (goto _label)))

(event `/Game/Blueprints/Interface/I_InteractivePlot.SelectOff`
  (params (Name :type String))
  (if (`KismetStringLibrary.EqualEqual_StrStr` Name (`KismetSystemLibrary.GetObjectName` self))
    (set `self.Selected` false)))

(event `/Game/Blueprints/Interface/I_InteractivePlot.SelectOn`
  (params (Name :type String))
  (if (`KismetStringLibrary.EqualEqual_StrStr` Name (`KismetSystemLibrary.GetObjectName` self))
    (set `self.Selected` true)))

(event `/Game/Blueprints/Interface/I_InteractivePlot.HoverOn`
  (params (Name :type String))
  (if (`KismetStringLibrary.EqualEqual_StrStr` Name (`KismetSystemLibrary.GetObjectName` self))
    (set `self.Hovered` true)
    (set `self.CurrentSelectionCounter` (`self.SelectionCounter`))))

(event `self.ReceiveBeginPlay`
  (`SceneComponent.SetVisibility` (`self.SelectedBox`) (`self.Hovered`) true)
  (bind _asvrgame_mode (cast `/Game/Blueprints/VRGameMode` (`GameplayStatics.GetGameMode`)))
  (set `self.VRGameMode` _asvrgame_mode))

(event `/Game/Blueprints/Interface/I_UpgradeAble.IUpgrade`
  (params (Name :type String))
  (if (`KismetStringLibrary.EqualEqual_StrStr` Name (`KismetSystemLibrary.GetObjectName` self))
    (`self.Upgrade`)))

(event `self.ReceiveTick`
  (params (DeltaSeconds :type "Float (single-precision)"))
  (bind _returnvalue (or (`self.Hovered`) (`self.Selected`)))
  (if (!= _returnvalue (`SceneComponent.IsVisible` (`self.SelectedBox`)))
    (`SceneComponent.SetVisibility` (`self.SelectedBox`) _returnvalue true))
  (if (and (`self.Hovered`) (> (`self.CurrentSelectionCounter`) 0.0))
    (set `self.CurrentSelectionCounter` (- (`self.CurrentSelectionCounter`) (`GameplayStatics.GetWorldDeltaSeconds`)))
    (elif (not (`self.Selected`))
      (set `self.Hovered` false))))

(fn `SetVisibility`
  (for (_ _array_index) (`self.UpgradeLevelsRoots`)
    (`SceneComponent.SetVisibility` (`|GetArrayItem` (`self.UpgradeLevelsRoots`) _array_index) (== _array_index (`self.CurrentLevel`)) true)))

(fn `Upgrade`
  (locals (Deleted :type Boolean))
  (if (< (+ (`self.CurrentLevel`) 1) (`KismetArrayLibrary.Array_Length` (`self.UpgradeLevelsRoots`)))
    (`/Engine/EditorBlueprintResources/StandardMacros.IncrementInt` (`self.CurrentLevel`)
      (:`  `
        (`self.SetVisibility`)))))

(fn `UserConstructionScript`)