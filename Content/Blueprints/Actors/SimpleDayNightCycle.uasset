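; Day-night cycle actor that advances an in-game hour on Tick, scaled so a full day lasts a configurable number of real minutes.
; The hour wraps at 24 and sets the pitch of the Sun and Moon actors, kept 180 degrees apart.
; Crossing the fixed day/night hour thresholds sends start messages to VRGameMode.
; Sky dome refresh and elapsed-time tracking nodes exist but never run.
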(event `self.ReceiveBeginPlay`
  (bind _output_get (set `self.OneDay` (* (`self.DaylengthInMinutes`) 60.0)))
  (set `self.OneHour` (/ _output_get 24.0))
  (bind _asvrgame_mode (cast `/Game/Blueprints/VRGameMode` (`GameplayStatics.GetGameMode`)))
  (set `self.VRGameMode` _asvrgame_mode))

(event `self.ReceiveTick`
  (params (DeltaSeconds :type "Float (single-precision)"))
  (bind _hour (`self.Hour`))
  (bind _vrgamemode (`self.VRGameMode`))
  (bind _hour_2 (`self.Hour`))
  (bind _returnvalue (and (> _hour_2 7.5) (< _hour_2 18.0)))
  (if (!= (`self.IsDay`) _returnvalue)
    (bind _output_get (set `self.IsDay` _returnvalue))
    (if _output_get
      (message `/Game/Blueprints/Interface/I_NightDayCall.DayStart` _vrgamemode)
      (else
        (message `/Game/Blueprints/Interface/I_NightDayCall.NightStart` _vrgamemode)))
    (else
      (if (>= _hour 24.0)
        (set `self.Hour` 0.0))
      (bind _output_get_2 (set `self.Hour` (+ _hour (/ DeltaSeconds (`self.OneHour`)))))
      (bind _output_get_3 (set `self.SunAngle` (+ (* (/ _output_get_2 6.0) 90.0) 90.0)))
      (`self.K2_SetActorRotation` (`self.Sun`) (`KismetMathLibrary.MakeRotator` 0.0 _output_get_3) false)
      (`self.K2_SetActorRotation` (`self.Moon`) (`KismetMathLibrary.MakeRotator` 0.0 (+ _output_get_3 180.0)) false))))

(fn `UserConstructionScript`)