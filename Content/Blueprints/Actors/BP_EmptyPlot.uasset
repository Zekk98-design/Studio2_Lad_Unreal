(event `self.ReceiveBeginPlay`
  (`SceneComponent.SetVisibility` (`self.SelectedBox`) (`self.Hovered`) true))

(event `self.ReceiveTick`
  (params (DeltaSeconds :type "Float (single-precision)"))
  (bind _returnvalue (or (`self.Hovered`) (`self.Selected`)))
  (if (!= (`SceneComponent.IsVisible` (`self.SelectedBox`)) _returnvalue)
    (`SceneComponent.SetVisibility` (`self.SelectedBox`) _returnvalue true)
    (`KismetSystemLibrary.PrintString` "visible"))
  (if (`self.Selected`)
    (`KismetSystemLibrary.PrintString` "--------------"))
  (if (and (> (`self.CurrentSelectionCounter`) 0.0) (`self.Hovered`))
    (set `self.CurrentSelectionCounter` (- (`self.CurrentSelectionCounter`) (`GameplayStatics.GetWorldDeltaSeconds`)))
    (elif (not (`self.Selected`))
      (`self.OffHover`))))

(fn `Build`
  (params (BuildingType :type Name) (BuildingID :type Integer))
  (switch `name` BuildingType
    (:`Housing`
      ;[1 1 1] Housing
      (`|SpawnActorFromClass` (`|GetArrayItem` (`self.Houses`) BuildingID) (`SceneComponent.K2_GetComponentToWorld` (`self.DefaultSceneRoot`)) "Undefined" "OverrideRootScale" null null)
      (`self.K2_DestroyActor`))
    (:`Storage`
      (`|SpawnActorFromClass` (`|GetArrayItem` (`self.Storage`) BuildingID) (`SceneComponent.K2_GetComponentToWorld` (`self.DefaultSceneRoot`)) "Undefined" "OverrideRootScale" null null)
      (`self.K2_DestroyActor`))))

(fn `OffHover`
  (set `self.Hovered` false))

(fn `OffSelect`
  (set `self.Selected` false))

(fn `OnHover`
  (set `self.Hovered` true)
  (set `self.CurrentSelectionCounter` (`self.SelectionCounter`)))

(fn `OnSelect`
  (set `self.Selected` true))

(fn `UserConstructionScript`)