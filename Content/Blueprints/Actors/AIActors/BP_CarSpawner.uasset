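; BP_CarSpawner is an actor that repeatedly spawns BP_AICar vehicles at random intervals.
; Tick runs a Delay between the min and max timer values, acting as the spawn loop.
; Each car spawns at the Billboard's location and rotation at reduced scale, then receives FirstWaypoint as its StartingWaypoint.
; A TextRender label is hidden on BeginPlay.
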(event `self.ReceiveBeginPlay`
  (`SceneComponent.SetVisibility` (`self.TextRender`) false false))

(event `self.ReceiveTick`
  (params (DeltaSeconds :type "Float (single-precision)"))
  (bind (_returnvalue_location _returnvalue_rotation) (`KismetMathLibrary.BreakTransform` (`SceneComponent.K2_GetComponentToWorld` (`self.Billboard`))))
  (`KismetSystemLibrary.Delay` (`KismetMathLibrary.RandomFloatInRange` (`self.MinCarSpawnTimer`) (`self.MaxCarSpawnTimer`)))
  (bind _returnvalue (`|SpawnActorFromClass` "/Game/Blueprints/Actors/AIActors/BP_AICar.BP_AICar_C" (`KismetMathLibrary.MakeTransform` _returnvalue_location _returnvalue_rotation (0.1 0.1 0.1)) "Undefined" "OverrideRootScale" null null))
  (set `/Game/Blueprints/Actors/AIActors/BP_AICar.StartingWaypoint` (`self.FirstWaypoint`) _returnvalue))

(fn `UserConstructionScript`)