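; AI car actor that drives toward a waypoint and can be grabbed by a hand.
; Tick eases Cube rotation toward the waypoint, seeded from StartingWaypoint, and moves it MaxSpeed units per frame, without delta-time scaling.
; Pickup toggles physics and hand attachment; once grabbed, driving stops for good and the car is destroyed after ten seconds.
; SetHighlight drives a custom-depth stencil highlight, which Tick clears unless refreshed.
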(event `self.ReceiveBeginPlay`
  (bind _startingwaypoint (`self.StartingWaypoint`))
  (`KismetSystemLibrary.Delay` 0.02)
  (`/Engine/EditorBlueprintResources/StandardMacros.IsValid` _startingwaypoint
    (:`Is Valid`
      (set `self.Waypoint` (`self.K2_GetActorLocation` _startingwaypoint)))))

(event `self.ReceiveTick`
  (params (DeltaSeconds :type "Float (single-precision)"))
  (bind _staticmesh (`self.StaticMesh`))
  (bind _cube (`self.Cube`))
  (bind _cube_2 (`self.Cube`))
  (bind _returnvalue (- 0.0 (`self.HighlightCountdown`)))
  (bind _returnvalue_2 (`SceneComponent.K2_GetComponentLocation` _cube_2))
  (bind _returnvalue_3 (`KismetMathLibrary.GetDirectionUnitVector` _returnvalue_2 (`self.Waypoint`)))
  (if (< _returnvalue 0.0)
    (set `self.HighlightCountdown` _returnvalue)
    (else
      (`PrimitiveComponent.SetRenderCustomDepth` _staticmesh false)
      (`PrimitiveComponent.SetCustomDepthStencilValue` _staticmesh 0)))
  (if (`self.boolPickedup`)
    (`KismetSystemLibrary.Delay` 10.0)
    (`self.K2_DestroyActor`)
    (else
      (`SceneComponent.K2_SetWorldRotation` _cube_2 (`KismetMathLibrary.RLerp` (`SceneComponent.K2_GetComponentRotation` _cube) (`KismetMathLibrary.FindLookAtRotation` (`SceneComponent.K2_GetComponentLocation` _cube) (`self.Waypoint`)) 0.1) false false)
      (`SceneComponent.K2_SetWorldLocation` (`self.Cube`) (+ (* _returnvalue_3 (/ (`self.MaxSpeed`) (`KismetMathLibrary.VSize` _returnvalue_3))) _returnvalue_2) false false))))

(event `/Game/Blueprints/Interface/I_Pickupable.Pickup`
  (params (Hand :type "SceneComponent Object Reference") (bHolding :type Boolean))
  (if bHolding
    (`PrimitiveComponent.SetSimulatePhysics` (`self.StaticMesh`) false)
    (`SceneComponent.K2_AttachToComponent` (`self.K2_GetRootComponent`) Hand "None" "KeepWorld" "KeepWorld" "KeepWorld" false)
    (set `self.boolPickedup` true)
    (else
      (`PrimitiveComponent.SetSimulatePhysics` (`self.StaticMesh`) true)
      (`self.K2_DetachFromActor` "KeepWorld" "KeepWorld" "KeepWorld")
      (`KismetSystemLibrary.PrintString` "Hello"))))

(event `/Game/Blueprints/Interface/I_Pickupable.SetHighlight`
  (params (Highlight :type Boolean))
  (bind _staticmesh (`self.StaticMesh`))
  (`PrimitiveComponent.SetRenderCustomDepth` _staticmesh Highlight)
  (`PrimitiveComponent.SetCustomDepthStencilValue` _staticmesh 2)
  (set `self.HighlightCountdown` 0.1))

(fn `UserConstructionScript`)