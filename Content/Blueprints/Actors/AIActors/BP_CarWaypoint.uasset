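; BP_CarWaypoint is a waypoint actor that routes AI cars through a network of linked waypoints.
; When a BP_AICar overlaps its Box, it sets the car's Waypoint to the location of a random entry in ConnectedWaypoints, or destroys the car if the checked entry is invalid.
; The validity check and the assignment roll separate random indices, so they can pick different entries.
; Its TextRender is hidden at BeginPlay.
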(event `self.ReceiveBeginPlay`
  (`SceneComponent.SetVisibility` (`self.TextRender`) false false))

(event `self.Box.OnComponentBeginOverlap`
  (params (OverlappedComponent :type "PrimitiveComponent Object Reference") (OtherActor :type "Actor Object Reference") (OtherComp :type "PrimitiveComponent Object Reference") (OtherBodyIndex :type Integer) (bFromSweep :type Boolean) (SweepResult :type "HitResult Structure (by ref)"))
  (bind _connectedwaypoints (`self.ConnectedWaypoints`))
  (bind _output (`|GetArrayItem` _connectedwaypoints (`KismetMathLibrary.RandomIntegerInRange` 0 (- (`KismetArrayLibrary.Array_Length` _connectedwaypoints) 1))))
  (bind _asbp_aicar (cast `/Game/Blueprints/Actors/AIActors/BP_AICar` OtherActor))
  (`/Engine/EditorBlueprintResources/StandardMacros.IsValid` _output
    (:`Is Valid`
      (set `/Game/Blueprints/Actors/AIActors/BP_AICar.Waypoint` (`self.K2_GetActorLocation` _output) _asbp_aicar))
    (:`Is Not Valid`
      (`self.K2_DestroyActor` _asbp_aicar))))

(fn `UserConstructionScript`)