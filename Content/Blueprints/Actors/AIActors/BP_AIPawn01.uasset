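; Scaled-down civilian AI pawn that walks to a random shop, clinic, research lab or housing building and destroys itself on arrival.
; SetTarget picks the building, recursing if none of that type exists; BeginPlay writes its position to the blackboard.
; Delayed Tick runs the behavior tree, feeds speed to the animation and accumulates slow-movement time.
; Being slow too long triggers one retarget, which leaves the blackboard unchanged, then destruction.
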(event `self.ReceiveBeginPlay`
  (bind _charactermovement (`self.CharacterMovement`))
  (bind _returnvalue_x (`KismetMathLibrary.BreakVector` (`SceneComponent.K2_GetComponentScale` (`self.CapsuleComponent`))))
  (`SceneComponent.SetWorldScale3D` (`self.CapsuleComponent`) (0.2 0.2 0.2))
  (set `CharacterMovementComponent.MaxWalkSpeed` (* (* (`MovementComponent.GetMaxSpeed` _charactermovement) _returnvalue_x) (`self.SpeedMuliti`)) _charactermovement)
  (bind _asmale_civilian_bp (cast `/Game/Assets/Charcters/Male_civilian_bp` (`SkeletalMeshComponent.GetAnimInstance` (`self.Mesh`))))
  (set `self.Animation` _asmale_civilian_bp)
  (`self.SetTarget`)
  (`self.SpawnDefaultController`)
  (bind _blackboardcomponent (`AIController.UseBlackboard` (`AIBlueprintHelperLibrary.GetAIController` (`self.GetController`)) "/Game/Blueprints/AI/BB_PawnAI.BB_PawnAI"))
  (`BlackboardComponent.SetValueAsVector` _blackboardcomponent "BuildingDestination" (`self.TargetPosition`)))

(event `self.ReceiveTick`
  (params (DeltaSeconds :type "Float (single-precision)"))
  (`KismetSystemLibrary.Delay` 0.2)
  (if (< (`KismetMathLibrary.Vector_Distance` (`self.TargetPosition`) (`SceneComponent.K2_GetComponentLocation` (`self.CapsuleComponent`))) (`self.FinishDistance`))
    (`self.K2_DestroyActor`)
    (else
      (`/Game/Assets/Charcters/Male_civilian_bp.SetSpeed` (`self.Animation`) (* (/ (`KismetMathLibrary.VSize` (`self.GetVelocity`)) (`MovementComponent.GetMaxSpeed` (`self.CharacterMovement`))) 100.0))
      (`AIController.RunBehaviorTree` (`AIBlueprintHelperLibrary.GetAIController` (`self.GetController`)) "/Game/Blueprints/AI/T_PawnAI.T_PawnAI")
      (if (< (* (/ (`KismetMathLibrary.VSize` (`self.GetVelocity`)) (`MovementComponent.GetMaxSpeed` (`self.CharacterMovement`))) 100.0) 40.0)
        (set `self.ChangeTargetTimer` (+ (`self.ChangeTargetTimer`) 0.2))
        (if (> (`self.ChangeTargetTimer`) 3.0)
          (if (or (> (`self.ChangeTargetTimer`) 5.0) (`self.Reset`))
            (`KismetSystemLibrary.PrintString` "KMS")
            (`self.K2_DestroyActor`)
            (else
              (`self.SetTarget`)
              (set `self.Reset` true)
              (set `self.ChangeTargetTimer` 0.0)
              (`KismetSystemLibrary.PrintString` "Reset Target"))))))))

(fn `GetRandomTarget`
  (params (TargetArray :type "Array of Actor Object Reference (by ref)"))
  (returns (Output :type "Actor Object Reference"))
  (bind _returnvalue (`KismetArrayLibrary.Array_Length` TargetArray))
  (if (> _returnvalue 0)
    (return (`|GetArrayItem` TargetArray (`KismetMathLibrary.RandomIntegerInRange` 0 (- _returnvalue 1))))
    (else
      (`self.SetTarget`))))

(fn `SetTarget`
  (switch `int` (`KismetMathLibrary.RandomIntegerInRange` 0 3)
    (:`Default`
      (`self.SetTarget`))
    (:`0`
      (bind _outactors (`GameplayStatics.GetAllActorsOfClass` "/Game/Blueprints/Actors/Buildings/BP_Shops.BP_Shops_C"))
      (bind _output (`self.GetRandomTarget` _outactors))
      (bind _asbp_shops (cast `/Game/Blueprints/Actors/Buildings/BP_Shops` _output))
      (set `self.TargetPosition` (`SceneComponent.K2_GetComponentLocation` (`/Game/Blueprints/Actors/Buildings/BP_Shops.Billboard` _asbp_shops))))
    (:`1`
      (bind _outactors_2 (`GameplayStatics.GetAllActorsOfClass` "/Game/Blueprints/Actors/Buildings/BP_Clinic.BP_Clinic_C"))
      (bind _output_2 (`self.GetRandomTarget` _outactors_2))
      (bind _asbp_clinic (cast `/Game/Blueprints/Actors/Buildings/BP_Clinic` _output_2))
      (set `self.TargetPosition` (`SceneComponent.K2_GetComponentLocation` (`/Game/Blueprints/Actors/Buildings/BP_Clinic.Billboard` _asbp_clinic))))
    (:`2`
      (bind _outactors_3 (`GameplayStatics.GetAllActorsOfClass` "/Game/Blueprints/Actors/Buildings/BP_ResearchLab.BP_ResearchLab_C"))
      (bind _output_3 (`self.GetRandomTarget` _outactors_3))
      (bind _asbp_research_lab (cast `/Game/Blueprints/Actors/Buildings/BP_ResearchLab` _output_3))
      (set `self.TargetPosition` (`SceneComponent.K2_GetComponentLocation` (`/Game/Blueprints/Actors/Buildings/BP_ResearchLab.Billboard` _asbp_research_lab))))
    (:`3`
      (bind _outactors_4 (`GameplayStatics.GetAllActorsOfClass` "/Game/Blueprints/Actors/Buildings/BP_Housing.BP_Housing_C"))
      (bind _output_4 (`self.GetRandomTarget` _outactors_4))
      (bind _asbp_housing (cast `/Game/Blueprints/Actors/Buildings/BP_Housing` _output_4))
      (set `self.TargetPosition` (`SceneComponent.K2_GetComponentLocation` (`/Game/Blueprints/Actors/Buildings/BP_Housing.Billboard` _asbp_housing))))))

(fn `UserConstructionScript`)