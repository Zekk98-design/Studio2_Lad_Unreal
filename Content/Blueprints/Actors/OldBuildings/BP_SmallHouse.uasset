(event `self.ReceiveTick`
  (params (DeltaSeconds :type "Float (single-precision)"))
  (if (and (> (`self.CurrentSelectionCounter`) 0.0) (`self.Selected`))
    (set `self.CurrentSelectionCounter` (- (`self.CurrentSelectionCounter`) DeltaSeconds))
    (else
      (`self.OffSelect`))))

(fn `Build`
  (params (BuildingType :type Name) (BuildingName :type Name) (BuildingLevel :type Integer))
  (locals (Building_Name :type Name) (Building_Level :type Integer))
  (bind _building_name (`local.Building_Name`))
  (switch `name` BuildingType
    (:`Housing`
      (switch `name` _building_name
        (:`SmallHouse`
          (`PawnAction.CreateActionInstance` null))))
    (:`Storage`
      (switch `name` _building_name))
    (:`Defence`
      (switch `name` _building_name))
    (:`Public Buildings`
      (switch `name` _building_name))))

(fn `OffSelect`
  (`SceneComponent.SetVisibility` (`self.SelectedBox`) false true)
  (set `self.Selected` false))

(fn `OnSelect`
  (set `self.Selected` true)
  (set `self.CurrentSelectionCounter` (`self.SelectionCounter`))
  (if (!= (`self.Selected`) (`SceneComponent.IsVisible` (`self.SelectedBox`)))
    (`SceneComponent.SetVisibility` (`self.SelectedBox`) (`self.Selected`) true)))

(fn `UserConstructionScript`)