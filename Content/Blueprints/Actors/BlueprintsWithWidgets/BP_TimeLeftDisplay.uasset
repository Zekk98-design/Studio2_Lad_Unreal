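; BP_TimeLeftDisplay is an in-world widget actor that hosts the W_TimeLeft display and shows the game-over message on a loss.
; It caches the VR pawn shortly after BeginPlay, then billboards the widget toward it every tick using a look-at rotation with 180-degree roll and pitch offsets.
; GameLose passes the lose text into W_TimeLeft and sets its game-over flag.
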(event `self.ReceiveBeginPlay`
  (`KismetSystemLibrary.Delay` 0.2)
  (bind _asvrpawn (cast `/Game/Blueprints/VRPawn` (`GameplayStatics.GetPlayerPawn` 0)))
  (set `self.PlayerPawn` _asvrpawn))

(event `self.ReceiveTick`
  (params (DeltaSeconds :type "Float (single-precision)"))
  (bind _playerpawn (`self.PlayerPawn`))
  (bind (_returnvalue_roll _returnvalue_pitch _returnvalue_yaw) (`KismetMathLibrary.BreakRotator` (`KismetMathLibrary.FindLookAtRotation` (`self.K2_GetActorLocation` _playerpawn) (`SceneComponent.K2_GetComponentLocation` (`self.Widget`)))))
  (`/Engine/EditorBlueprintResources/StandardMacros.IsValid` _playerpawn
    (:`Is Valid`
      (`SceneComponent.K2_SetWorldRotation` (`self.Widget`) (`KismetMathLibrary.MakeRotator` (- _returnvalue_roll 180.0) (- _returnvalue_pitch 180.0) _returnvalue_yaw) false false))))

(event `/Game/Blueprints/Interface/I_LoseConditions.GameLose`
  (params (LoseText :type String))
  (bind _asw_time_left (cast `/Game/Blueprints/Widgets/W_TimeLeft` (`WidgetComponent.GetUserWidgetObject` (`self.Widget`))))
  (set `/Game/Blueprints/Widgets/W_TimeLeft.GameOverTest` LoseText _asw_time_left)
  (set `/Game/Blueprints/Widgets/W_TimeLeft.GameOver` true _asw_time_left))

(fn `UserConstructionScript`)