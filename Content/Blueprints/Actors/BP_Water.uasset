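; BP_Water is a water actor that sets up a recolorable water material on its Watergrid component.
; On BeginPlay it creates a dynamic instance of MTS_Water, assigns it to the grid and caches its "Main color" value.
; An unconnected chain would lerp that color toward bright green by CurrentRad over MaxRad and increment CurrentRad, but nothing triggers it.
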(event `self.ReceiveBeginPlay`
  (bind _returnvalue (`PrimitiveComponent.CreateDynamicMaterialInstance` (`self.Watergrid`) 0 "/Game/Assets/Water/MTS_Water.MTS_Water" "None"))
  (bind _output_get (set `self.DynamicMat` _returnvalue))
  (`PrimitiveComponent.SetMaterial` (`self.Watergrid`) 0 _output_get)
  (bind _returnvalue_2 (`MaterialInstanceDynamic.K2_GetVectorParameterValue` _returnvalue "Main color"))
  (set `self.CurrentWaterColor` _returnvalue_2))

(event `self.ReceiveTick`
  (params (DeltaSeconds :type "Float (single-precision)")))

(fn `UserConstructionScript`)