(event `/Game/Blueprints/Interface/I_InteractivePlot.SelectOff`
  (params (Name :type String))
  (if (`KismetStringLibrary.EqualEqual_StrStr` Name (`KismetSystemLibrary.GetObjectName` self))
    (set `self.Selected` false)))

(event `/Game/Blueprints/Interface/I_InteractivePlot.SelectOn`
  (params (Name :type String))
  (if (`KismetStringLibrary.EqualEqual_StrStr` Name (`KismetSystemLibrary.GetObjectName` self))
    (set `self.Selected` true)))

(event `/Game/Blueprints/Interface/I_InteractivePlot.HoverOn`
  (params (Name :type String))
  (if (`KismetStringLibrary.EqualEqual_StrStr` Name (`KismetSystemLibrary.GetObjectName` self))
    (set `self.Hovered` true)
    (set `self.CurrentSelectionCounter` (`self.SelectionCounter`))))

(event `/Game/Blueprints/Interface/I_InteractivePlot.IBuild`
  (params (IBuildingType :type Name) (IBuildingID :type Integer) (Name :type String))
  (if (`KismetStringLibrary.EqualEqual_StrStr` Name (`KismetSystemLibrary.GetObjectName` self))
    (`self.Build` IBuildingType IBuildingID)))

(event `/Game/Blueprints/Interface/I_InteractivePlot.GetInteractiveValues`
  (bind _asvrpawn (cast `/Game/Blueprints/VRPawn` (`GameplayStatics.GetPlayerPawn` 0)))
  (`/Game/Blueprints/Interface/I_InteractivePlot.SendInteractiveValues` _asvrpawn "EmptyPlot" 0))

(event `self.ReceiveBeginPlay`
  (`SceneComponent.SetVisibility` (`self.SelectedBox`) (`self.Hovered`) true))

(event `self.ReceiveTick`
  (params (DeltaSeconds :type "Float (single-precision)"))
  (bind _returnvalue (or (`self.Hovered`) (`self.Selected`)))
  (if (!= _returnvalue (`SceneComponent.IsVisible` (`self.SelectedBox`)))
    (`SceneComponent.SetVisibility` (`self.SelectedBox`) _returnvalue true)
    (if (not (`self.Selected`))
      (`self.GhostBuilding` "")))
  (if (and (`self.Hovered`) (> (`self.CurrentSelectionCounter`) 0.0))
    (set `self.CurrentSelectionCounter` (- (`self.CurrentSelectionCounter`) (`GameplayStatics.GetWorldDeltaSeconds`)))
    (elif (not (`self.Selected`))
      (set `self.Hovered` false))))

(fn `Build`
  (params (BuildingType :type Name) (BuildingID :type Integer))
  (locals (LocBuildingType :type Name) (LocBuildingID :type Integer))
  (set `local.LocBuildingID` BuildingID)
  (switch `name` BuildingType
    (:`House`
      ;[1 1 1] Housing
      (bind _returnvalue (`|SpawnActorFromClass` "/Game/Blueprints/Actors/InteractiveBuildings/BP_Housing.BP_Housing_C" (`SceneComponent.K2_GetComponentToWorld` (`self.DefaultSceneRoot`)) "Undefined" "OverrideRootScale" null null))
      (set `/Game/Blueprints/Actors/InteractiveBuildings/BP_Housing.CurrentLevel` (`local.LocBuildingID`) _returnvalue)
      (`self.K2_DestroyActor`))
    (:`Storage`
      ;[1 1 1] Storage
      (bind _returnvalue_2 (`|SpawnActorFromClass` "/Game/Blueprints/Actors/InteractiveBuildings/BP_Storage.BP_Storage_C" (`SceneComponent.K2_GetComponentToWorld` (`self.DefaultSceneRoot`)) "Undefined" "OverrideRootScale" null null))
      (set `/Game/Blueprints/Actors/InteractiveBuildings/BP_Storage.CurrentLevel` (`local.LocBuildingID`) _returnvalue_2)
      (`self.K2_DestroyActor`))
    (:`Entertainment`
      ;[1 1 1] Entertainment
      (bind _returnvalue_3 (`|SpawnActorFromClass` "/Game/Blueprints/Actors/InteractiveBuildings/Removed/BP_Entertainment.BP_Entertainment_C" (`SceneComponent.K2_GetComponentToWorld` (`self.DefaultSceneRoot`)) "Undefined" "OverrideRootScale" null null))
      (set `/Game/Blueprints/Actors/InteractiveBuildings/Removed/BP_Entertainment.CurrentLevel` (`local.LocBuildingID`) _returnvalue_3)
      (`self.K2_DestroyActor`))
    (:`ResearchLab`
      ;[1 1 1] Research
      (bind _returnvalue_4 (`|SpawnActorFromClass` "/Game/Blueprints/Actors/InteractiveBuildings/BP_ResearchLab.BP_ResearchLab_C" (`SceneComponent.K2_GetComponentToWorld` (`self.DefaultSceneRoot`)) "Undefined" "OverrideRootScale" null null))
      (set `/Game/Blueprints/Actors/InteractiveBuildings/BP_ResearchLab.CurrentLevel` (`local.LocBuildingID`) _returnvalue_4)
      (`self.K2_DestroyActor`))
    (:`Clinic`
      ;[1 1 1] Clinic
      (bind _returnvalue_5 (`|SpawnActorFromClass` "/Game/Blueprints/Actors/InteractiveBuildings/BP_Clinic.BP_Clinic_C" (`SceneComponent.K2_GetComponentToWorld` (`self.DefaultSceneRoot`)) "Undefined" "OverrideRootScale" null null))
      (set `/Game/Blueprints/Actors/InteractiveBuildings/BP_Clinic.CurrentLevel` (`local.LocBuildingID`) _returnvalue_5)
      (`self.K2_DestroyActor`))
    (:`Shopping`
      ;[1 1 1] Shopping
      (bind _returnvalue_6 (`|SpawnActorFromClass` "/Game/Blueprints/Actors/InteractiveBuildings/BP_Shops.BP_Shops_C" (`SceneComponent.K2_GetComponentToWorld` (`self.DefaultSceneRoot`)) "Undefined" "OverrideRootScale" null null))
      (set `/Game/Blueprints/Actors/InteractiveBuildings/BP_Shops.CurrentLevel` (`local.LocBuildingID`) _returnvalue_6)
      (`self.K2_DestroyActor`))))

(fn `GhostBuilding`
  (params (Name :type String) (Level :type Integer))
  (bind _shops (`self.Shops`))
  (bind _house (`self.House`))
  (bind _storage (`self.Storage`))
  (bind _hospital (`self.Hospital`))
  (bind _researchlab (`self.ResearchLab`))
  (`SceneComponent.SetVisibility` (`self.House`) false false)
  (`SceneComponent.SetVisibility` (`self.Storage`) false false)
  (`SceneComponent.SetVisibility` (`self.Hospital`) false false)
  (`SceneComponent.SetVisibility` (`self.ResearchLab`) false false)
  (`SceneComponent.SetVisibility` (`self.Shops`) false false)
  (switch `string` Name
    (:`House`
      (`StaticMeshComponent.SetStaticMesh` _house (`|GetArrayItem` (`self.GhostHouse`) Level))
      (`SceneComponent.SetVisibility` _house true false))
    (:`Storage`
      (`StaticMeshComponent.SetStaticMesh` _storage (`|GetArrayItem` (`self.GhostStorage`) Level))
      (`SceneComponent.SetVisibility` _storage true false))
    (:`Clinic`
      (`StaticMeshComponent.SetStaticMesh` _hospital (`|GetArrayItem` (`self.GhostHospital`) Level))
      (`SceneComponent.SetVisibility` _hospital true false))
    (:`ResearchLab`
      (`StaticMeshComponent.SetStaticMesh` _researchlab (`|GetArrayItem` (`self.GhostResearchLab`) Level))
      (`SceneComponent.SetVisibility` _researchlab true false))
    (:`Shopping`
      (`StaticMeshComponent.SetStaticMesh` _shops (`|GetArrayItem` (`self.GhostShops`) Level))
      (`SceneComponent.SetVisibility` _shops true false))))

(fn `UserConstructionScript`)