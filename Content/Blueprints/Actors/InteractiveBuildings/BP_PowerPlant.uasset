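; Interactive power plant building that players hover, select and upgrade, and that raises or lowers the game mode's current power.
; Name-filtered events step power up or down, clamped to a MaxPower read from DT_Powerplant for the current level.
; Upgrading shows that level's mesh root, publishes the level to VRGameMode and reloads MaxPower; Downgrade skips that reload.
; Tick drives the selection box, expiring hover on a countdown unless selected.
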(event `/Game/Blueprints/Interface/I_PowerPlant.IncreasePower`
  (params (Name :type String))
  (bind _vrgamemode (`self.VRGameMode`))
  ;[1 1 1] Managing Power
  (if (`KismetStringLibrary.EqualEqual_StrStr` Name (`KismetSystemLibrary.GetObjectName` self))
    (bind _output_get (set `/Game/Blueprints/VRGameMode.CurrentPower` (`KismetMathLibrary.FClamp` (+ (`/Game/Blueprints/VRGameMode.CurrentPower` _vrgamemode) 10.0) 0.0 (`self.MaxPower`)) _vrgamemode))
    (`KismetSystemLibrary.PrintString` (`KismetStringLibrary.Conv_DoubleToString` _output_get))))

(event `/Game/Blueprints/Interface/I_PowerPlant.DecreasePower`
  (params (Name :type String))
  (bind _vrgamemode (`self.VRGameMode`))
  ;[1 1 1] Managing Power
  (if (`KismetStringLibrary.EqualEqual_StrStr` Name (`KismetSystemLibrary.GetObjectName` self))
    (bind _output_get (set `/Game/Blueprints/VRGameMode.CurrentPower` (`KismetMathLibrary.FClamp` (- (`/Game/Blueprints/VRGameMode.CurrentPower` _vrgamemode) 10.0) 0.0 (`self.MaxPower`)) _vrgamemode))
    (`KismetSystemLibrary.PrintString` (`KismetStringLibrary.Conv_DoubleToString` _output_get))))

(event `/Game/Blueprints/Interface/I_InteractivePlot.SelectOff`
  (params (Name :type String))
  ;[1 1 1] Selecting
  (if (`KismetStringLibrary.EqualEqual_StrStr` Name (`KismetSystemLibrary.GetObjectName` self))
    (set `self.Selected` false)))

(event `/Game/Blueprints/Interface/I_InteractivePlot.SelectOn`
  (params (Name :type String))
  ;[1 1 1] Selecting
  (if (`KismetStringLibrary.EqualEqual_StrStr` Name (`KismetSystemLibrary.GetObjectName` self))
    (set `self.Selected` true)))

(event `self.ReceiveBeginPlay`
  (`SceneComponent.SetVisibility` (`self.SelectedBox`) (`self.Hovered`) true)
  (`KismetArrayLibrary.Array_Add` (`self.UpgradeLevelsRoots`) (`self.UpgradeLevel0`))
  (`KismetArrayLibrary.Array_Add` (`self.UpgradeLevelsRoots`) (`self.UpgradeLevel1`))
  (`KismetArrayLibrary.Array_Add` (`self.UpgradeLevelsRoots`) (`self.UpgradeLevel2`))
  (`KismetArrayLibrary.Array_Add` (`self.UpgradeLevelsRoots`) (`self.UpgradeLevel3`))
  (`self.SetVisibility`)
  (bind _asvrgame_mode (cast `/Game/Blueprints/VRGameMode` (`GameplayStatics.GetGameMode`)))
  (bind _output_get (set `self.VRGameMode` _asvrgame_mode))
  (set `/Game/Blueprints/VRGameMode.PowerStationLevel` (`self.CurrentLevel`) _output_get)
  (`self.SetVariables`))

(event `/Game/Blueprints/Interface/I_InteractivePlot.HoverOn`
  (params (Name :type String))
  ;[1 1 1] Selecting
  (if (`KismetStringLibrary.EqualEqual_StrStr` Name (`KismetSystemLibrary.GetObjectName` self))
    (set `self.Hovered` true)
    (set `self.CurrentSelectionCounter` (`self.SelectionCounter`))))

(event `/Game/Blueprints/Interface/I_UpgradeAble.IUpgrade`
  (params (Name :type String) (UpgradeLevel :type Integer))
  ;[1 1 1] Upgrade
  (if (`KismetStringLibrary.EqualEqual_StrStr` Name (`KismetSystemLibrary.GetObjectName` self))
    (`self.Upgrade`)))

(event `/Game/Blueprints/Interface/I_InteractivePlot.GetInteractiveValues`
  (bind _asvrpawn (cast `/Game/Blueprints/VRPawn` (`GameplayStatics.GetPlayerPawn` 0)))
  (`/Game/Blueprints/Interface/I_InteractivePlot.SendInteractiveValues` _asvrpawn "Powerplant" (`self.CurrentLevel`)))

(event `self.ReceiveTick`
  (params (DeltaSeconds :type "Float (single-precision)"))
  (bind _returnvalue (or (`self.Hovered`) (`self.Selected`)))
  (if (!= _returnvalue (`SceneComponent.IsVisible` (`self.SelectedBox`)))
    (`SceneComponent.SetVisibility` (`self.SelectedBox`) _returnvalue true))
  (if (and (`self.Hovered`) (> (`self.CurrentSelectionCounter`) 0.0))
    (set `self.CurrentSelectionCounter` (- (`self.CurrentSelectionCounter`) (`GameplayStatics.GetWorldDeltaSeconds`)))
    (elif (not (`self.Selected`))
      (set `self.Hovered` false))))

(fn `Downgrade`
  (if (> (`self.CurrentLevel`) 0)
    (`/Engine/EditorBlueprintResources/StandardMacros.DecrementInt` (`self.CurrentLevel`)
      (:`  `
        (`self.SetVisibility`)
        (set `/Game/Blueprints/VRGameMode.PowerStationLevel` (`self.CurrentLevel`) (`self.VRGameMode`))))))

(fn `SetVariables`
  (bind _returnvalue (`|GetDataTableRow` "/Game/Blueprints/DataManagement/DT_Powerplant.DT_Powerplant" (`KismetStringLibrary.Conv_StringToName` (`KismetStringLibrary.Concat_StrStr` "Powerplant" (`KismetStringLibrary.Conv_IntToString` (`self.CurrentLevel`)))))
    (:`then`
      (set `self.MaxPower` (`.MaxPower_7_3D513D7341BC352A89BD2A8833FDEFA0` (break `/Game/Blueprints/DataManagement/Struct_Powerplant` _returnvalue))))))

(fn `SetVisibility`
  (for (_ _array_index) (`self.UpgradeLevelsRoots`)
    (`SceneComponent.SetVisibility` (`|GetArrayItem` (`self.UpgradeLevelsRoots`) _array_index) (== _array_index (`self.CurrentLevel`)) true)))

(fn `Upgrade`
  (locals (Deleted :type Boolean))
  (if (< (+ (`self.CurrentLevel`) 1) (`KismetArrayLibrary.Array_Length` (`self.UpgradeLevelsRoots`)))
    (`/Engine/EditorBlueprintResources/StandardMacros.IncrementInt` (`self.CurrentLevel`)
      (:`  `
        (`self.SetVisibility`)
        (set `/Game/Blueprints/VRGameMode.PowerStationLevel` (`self.CurrentLevel`) (`self.VRGameMode`))
        (`self.SetVariables`)))))

(fn `UserConstructionScript`)