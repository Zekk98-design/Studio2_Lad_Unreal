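; Uranium spawner building that a VR player toggles on and off with a physical button, buying uranium on a timer while active.
; Overlap of a VRPawn with the button box, gated by a cooldown, flips Active, moves the button and swaps the on/off lights.
; While active, Tick runs a speed-scaled countdown that calls CreateBox, which spawns a randomly rotated BP_Uranium at the spawn point and deducts its price from VRGameMode Money if affordable.
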(event `self.ReceiveBeginPlay`
  (`SceneComponent.K2_SetRelativeLocation` (`self.Button`) (0.0 0.0 615.0) false false)
  (`SceneComponent.SetVisibility` (`self.PointLightOff`) true false)
  (bind _asvrgame_mode (cast `/Game/Blueprints/VRGameMode` (`GameplayStatics.GetGameMode`)))
  (set `self.VRGamemode` _asvrgame_mode))

(event `self.ReceiveTick`
  (params (DeltaSeconds :type "Float (single-precision)"))
  (set `self.CurrentButtonCooldown` (- (`self.CurrentButtonCooldown`) DeltaSeconds))
  (if (`self.Active`)
    (set `self.CurrentSpawnTimer` (- (`self.CurrentSpawnTimer`) (* DeltaSeconds (`self.SpeedModifier`))))
    (`KismetSystemLibrary.Delay` 0.1)
    (if (<= (`self.CurrentSpawnTimer`) 0.0)
      (`self.CreateBox`)
      (set `self.CurrentSpawnTimer` (`self.SpawnTimer`)))))

(event `self.Box.OnComponentBeginOverlap`
  (params (OverlappedComponent :type "PrimitiveComponent Object Reference") (OtherActor :type "Actor Object Reference") (OtherComp :type "PrimitiveComponent Object Reference") (OtherBodyIndex :type Integer) (bFromSweep :type Boolean) (SweepResult :type "HitResult Structure (by ref)"))
  (if (<= (`self.CurrentButtonCooldown`) 0.0)
    (cast `/Game/Blueprints/VRPawn` OtherActor)
    (`self.ButtonPressed`)
    (set `self.CurrentButtonCooldown` (`self.ButtonCooldown`))))

(fn `ButtonPressed`
  (`SceneComponent.SetVisibility` (`self.PointLightOff`) false false)
  (`SceneComponent.SetVisibility` (`self.PointLightOn`) false false)
  (if (`self.Active`)
    (`SceneComponent.K2_SetRelativeLocation` (`self.Button`) (0.0 0.0 615.0) false false)
    (`SceneComponent.SetVisibility` (`self.PointLightOff`) true false)
    (else
      (`SceneComponent.K2_SetRelativeLocation` (`self.Button`) (0.0 0.0 575.0) false false)
      (`SceneComponent.SetVisibility` (`self.PointLightOn`) true false)))
  (set `self.Active` (not (`self.Active`))))

(fn `CreateBox`
  (bind _returnvalue (`KismetMathLibrary.RandomFloatInRange` 0.0 360.0))
  (bind _vrgamemode (`self.VRGamemode`))
  (bind _returnvalue_location (`KismetMathLibrary.BreakTransform` (`SceneComponent.K2_GetComponentToWorld` (`self.CrateSpawnpoint`))))
  (if (>= (- (`/Game/Blueprints/VRGameMode.Money` (`self.VRGamemode`)) (`self.PricePerBox`)) 0.0)
    (`|SpawnActorFromClass` "/Game/Blueprints/Actors/PickupObjects/BP_Uranium.BP_Uranium_C" (`KismetMathLibrary.MakeTransform` _returnvalue_location (`KismetMathLibrary.MakeRotator` _returnvalue _returnvalue _returnvalue) (2.0 2.0 2.0)) "Undefined" "OverrideRootScale" null null)
    (set `/Game/Blueprints/VRGameMode.Money` (- (`/Game/Blueprints/VRGameMode.Money` _vrgamemode) (`self.PricePerBox`)) _vrgamemode)))

(fn `UserConstructionScript`)