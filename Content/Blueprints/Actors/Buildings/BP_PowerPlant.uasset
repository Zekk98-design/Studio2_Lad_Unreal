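; Upgradeable power plant building for a VR city game that burns uranium into stored power and produces nuclear waste.
; Uranium entering the Sucker is lerped into the Destroyer, refilling storage, which Tick drains by game mode power draw to set whether the city is powered.
; Draw also fills a waste buffer that spawns barrel actors.
; Upgrade levels swap visible meshes and load limits from a data table; a player-facing widget shows storage.
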(event `/Game/Blueprints/Interface/I_UpgradeAble.GhostVisiblity`
  (params (Level :type Integer))
  (`self.GhostVisibility` Level))

(event `/Game/Blueprints/Interface/I_PowerPlant.IncreasePower`
  (params (Name :type String))
  ;[1 1 1] Managing Power
)

(event `/Game/Blueprints/Interface/I_PowerPlant.DecreasePower`
  (params (Name :type String))
  ;[1 1 1] Managing Power
)

(event `/Game/Blueprints/Interface/I_InteractivePlot.SelectOff`
  (params (Name :type String))
  ;[1 1 1] Selecting
  (if (`KismetStringLibrary.EqualEqual_StrStr` Name (`KismetSystemLibrary.GetObjectName` self))
    (set `self.Selected` false)))

(event `/Game/Blueprints/Interface/I_InteractivePlot.SelectOn`
  (params (Name :type String))
  ;[1 1 1] Selecting
  (if (`KismetStringLibrary.EqualEqual_StrStr` Name (`KismetSystemLibrary.GetObjectName` self))
    (set `self.Selected` true)))

(event `self.ReceiveBeginPlay`
  (`KismetSystemLibrary.Delay` 0.05)
  (`SceneComponent.SetVisibility` (`self.SelectedBox`) (`self.Hovered`) true)
  (`KismetArrayLibrary.Array_Add` (`self.UpgradeLevelsRoots`) (`self.UpgradeLevel0`))
  (`KismetArrayLibrary.Array_Add` (`self.UpgradeLevelsRoots`) (`self.UpgradeLevel1`))
  (`KismetArrayLibrary.Array_Add` (`self.UpgradeLevelsRoots`) (`self.UpgradeLevel2`))
  (`KismetArrayLibrary.Array_Add` (`self.UpgradeLevelsRoots`) (`self.UpgradeLevel3`))
  (`self.SetVisibility`)
  (bind _asvrgame_mode (cast `/Game/Blueprints/VRGameMode` (`GameplayStatics.GetGameMode`)))
  (bind _output_get (set `self.VRGameMode` _asvrgame_mode))
  (set `/Game/Blueprints/VRGameMode.PowerStationLevel` (`self.CurrentLevel`) _output_get)
  (`self.SetVariables`)
  (set `self.CurrentPowerStorage` (`self.MaxPower`)))

(event `/Game/Blueprints/Interface/I_InteractivePlot.HoverOn`
  (params (Name :type String))
  ;[1 1 1] Selecting
  (if (`KismetStringLibrary.EqualEqual_StrStr` Name (`KismetSystemLibrary.GetObjectName` self))
    (set `self.Hovered` true)
    (set `self.CurrentSelectionCounter` (`self.SelectionCounter`))))

(event `/Game/Blueprints/Interface/I_UpgradeAble.IUpgrade`
  (params (Name :type String) (UpgradeLevel :type Integer))
  ;[1 1 1] Upgrade
  (if (`KismetStringLibrary.EqualEqual_StrStr` Name (`KismetSystemLibrary.GetObjectName` self))
    (`self.Upgrade` UpgradeLevel)))

(event `/Game/Blueprints/Interface/I_InteractivePlot.GetInteractiveValues`
  ;[1 1 1] Send Values to player pawn
  (bind _asvrpawn (cast `/Game/Blueprints/VRPawn` (`GameplayStatics.GetPlayerPawn` 0)))
  (`/Game/Blueprints/Interface/I_InteractivePlot.SendInteractiveValues` _asvrpawn "Powerplant" (`self.CurrentLevel`)))

(event `self.ReceiveTick`
  (params (DeltaSeconds :type "Float (single-precision)"))
  (bind _returnvalue (`KismetMathLibrary.RandomFloatInRange` 0.0 360.0))
  (bind _vrgamemode (`self.VRGameMode`))
  (bind _vrgamemode_2 (`self.VRGameMode`))
  (bind _returnvalue_2 (or (`self.Hovered`) (`self.Selected`)))
  (`|ExecutionSequence`
    (:`then_0`
      (`self.SuckObjects`)
      (if (!= _returnvalue_2 (`SceneComponent.IsVisible` (`self.SelectedBox`)))
        (`SceneComponent.SetVisibility` (`self.SelectedBox`) _returnvalue_2 true)
        (if (not (`self.Selected`))
          (`self.SetVisibility`)))
      (if (and (`self.Hovered`) (> (`self.CurrentSelectionCounter`) 0.0))
        (set `self.CurrentSelectionCounter` (- (`self.CurrentSelectionCounter`) (`GameplayStatics.GetWorldDeltaSeconds`)))
        (elif (not (`self.Selected`))
          (set `self.Hovered` false))))
    (:`then_1`
      (`KismetSystemLibrary.Delay` 0.2)
      ;[1 1 1] Managing Power
      (bind _output_get (set `self.CurrentPowerStorage` (`KismetMathLibrary.FClamp` (- (`self.CurrentPowerStorage`) (`/Game/Blueprints/VRGameMode.CurrentPowerDraw` (`self.VRGameMode`))) 0.0 (`self.MaxPower`))))
      (set `/Game/Blueprints/VRGameMode.CityPowered` (>= _output_get (`/Game/Blueprints/VRGameMode.PowerRequired` _vrgamemode_2)) _vrgamemode_2))
    (:`then_2`
      ;[1 1 1] Widget Lookat player
      (bind _asvrpawn (cast `/Game/Blueprints/VRPawn` (`GameplayStatics.GetPlayerPawn` 0)))
      (`SceneComponent.K2_SetWorldRotation` (`self.PowerDisplay`) (`KismetMathLibrary.FindLookAtRotation` (`SceneComponent.K2_GetComponentLocation` (`self.PowerDisplay`)) (`SceneComponent.K2_GetComponentLocation` (`/Game/Blueprints/VRPawn.Camera` _asvrpawn))) false false)
      ;[1 1 1] Set Widget varibles
      (`KismetSystemLibrary.Delay` 0.2)
      (bind _asw_power_plant_ui (cast `/Game/Blueprints/Widgets/W_PowerPlantUI` (`WidgetComponent.GetUserWidgetObject` (`self.PowerDisplay`))))
      (set `/Game/Blueprints/Widgets/W_PowerPlantUI.fCurrentStorage` (`self.CurrentPowerStorage`) _asw_power_plant_ui)
      (set `/Game/Blueprints/Widgets/W_PowerPlantUI.fMaxStorage` (`self.MaxPower`) _asw_power_plant_ui)
      (set `/Game/Blueprints/Widgets/W_PowerPlantUI.fPowerRequired` (`/Game/Blueprints/VRGameMode.PowerRequired` (`self.VRGameMode`)) _asw_power_plant_ui))
    (:`then_3`
      ;[1 1 1] CreatingNuclearWaste
      (`KismetSystemLibrary.Delay` 0.2)
      (bind _output_get_2 (set `self.WasteBuffer` (+ (`self.WasteBuffer`) (* (`/Game/Blueprints/VRGameMode.CurrentPowerDraw` _vrgamemode) (`/Game/Blueprints/VRGameMode.WasteEfficiency` _vrgamemode) (`/Game/Blueprints/VRGameMode.UpWatseMulti` _vrgamemode)))))
      (if (> _output_get_2 (`self.NuclearWasteBarrelSize`))
        (bind _returnvalue_3 (`|SpawnActorFromClass` "/Game/Blueprints/Actors/PickupObjects/BP_NuclearWaste.BP_NuclearWaste_C" (`KismetMathLibrary.MakeTransform` (`SceneComponent.K2_GetComponentLocation` (`self.NuclearWasteSpawn`)) (`KismetMathLibrary.MakeRotator` _returnvalue _returnvalue _returnvalue) (0.25 0.25 0.25)) "Undefined" "OverrideRootScale" null null))
        (set `/Game/Blueprints/Actors/PickupObjects/BP_NuclearWaste.WasteCarried` (`self.WasteBuffer`) _returnvalue_3)
        (set `self.WasteBuffer` 0.0)))))

(event `self.Sucker.OnComponentBeginOverlap`
  (params (OverlappedComponent :type "PrimitiveComponent Object Reference") (OtherActor :type "Actor Object Reference") (OtherComp :type "PrimitiveComponent Object Reference") (OtherBodyIndex :type Integer) (bFromSweep :type Boolean) (SweepResult :type "HitResult Structure (by ref)"))
  (`/Engine/EditorBlueprintResources/StandardMacros.IsValid` (`self.ObjectsInSucker`)
    (:`Is Not Valid`
      (bind _asbp_uranium (cast `/Game/Blueprints/Actors/PickupObjects/BP_Uranium` OtherActor))
      (set `self.ObjectsInSucker` _asbp_uranium))))

(event `self.Destroyer.OnComponentBeginOverlap`
  (params (OverlappedComponent :type "PrimitiveComponent Object Reference") (OtherActor :type "Actor Object Reference") (OtherComp :type "PrimitiveComponent Object Reference") (OtherBodyIndex :type Integer) (bFromSweep :type Boolean) (SweepResult :type "HitResult Structure (by ref)"))
  (bind _asbp_uranium (cast `/Game/Blueprints/Actors/PickupObjects/BP_Uranium` OtherActor))
  (set `self.ObjectsInSucker` null)
  (`self.K2_DestroyActor` _asbp_uranium)
  (set `self.CurrentPowerStorage` (`KismetMathLibrary.FClamp` (+ (`self.PowerGainedPerBox`) (`self.CurrentPowerStorage`)) 0.0 (`self.MaxPower`))))

(fn `CreateNuclearWaste`)

(fn `Downgrade`
  (if (> (`self.CurrentLevel`) 0)
    (`/Engine/EditorBlueprintResources/StandardMacros.DecrementInt` (`self.CurrentLevel`)
      (:`  `
        (`self.SetVisibility`)
        (set `/Game/Blueprints/VRGameMode.PowerStationLevel` (`self.CurrentLevel`) (`self.VRGameMode`))))))

(fn `GhostVisibility`
  (params (Level :type Integer))
  (for (_ _array_index) (`self.UpgradeLevelsRoots`)
    (`SceneComponent.SetVisibility` (`|GetArrayItem` (`self.UpgradeLevelsRoots`) _array_index) (== _array_index Level) true)))

(fn `SetVariables`
  (bind _returnvalue (`|GetDataTableRow` "/Game/Blueprints/DataManagement/DT_Powerplant.DT_Powerplant" (`KismetStringLibrary.Conv_StringToName` (`KismetStringLibrary.Concat_StrStr` "Powerplant" (`KismetStringLibrary.Conv_IntToString` (`self.CurrentLevel`)))))
    (:`then`
      (bind (_maxpower _wasteefficiency _powerefficiency _price _populationrequired _wastebarrelsize) (break `/Game/Blueprints/DataManagement/Struct_Powerplant` _returnvalue))
      (set `self.MaxPower` _maxpower)
      (set `self.NuclearWasteBarrelSize` _wastebarrelsize))))

(fn `SetVisibility`
  (for (_ _array_index) (`self.UpgradeLevelsRoots`)
    (`SceneComponent.SetVisibility` (`|GetArrayItem` (`self.UpgradeLevelsRoots`) _array_index) (== _array_index (`self.CurrentLevel`)) true)))

(fn `SuckObjects`
  (bind _objectsinsucker (`self.ObjectsInSucker`))
  (bind (_returnvalue_location _returnvalue_rotation) (`KismetMathLibrary.BreakTransform` (`SceneComponent.K2_GetComponentToWorld` (`self.Destroyer`))))
  (`/Engine/EditorBlueprintResources/StandardMacros.IsValid` (`self.ObjectsInSucker`)
    (:`Is Valid`
      (`PrimitiveComponent.SetSimulatePhysics` (`/Game/Blueprints/Actors/PickupObjects/BP_Uranium.StaticMesh` (`self.ObjectsInSucker`)) false)
      (`SceneComponent.K2_SetWorldTransform` (`/Game/Blueprints/Actors/PickupObjects/BP_Uranium.StaticMesh` _objectsinsucker) (`KismetMathLibrary.TLerp` (`SceneComponent.K2_GetComponentToWorld` (`/Game/Blueprints/Actors/PickupObjects/BP_Uranium.StaticMesh` _objectsinsucker)) (`KismetMathLibrary.MakeTransform` _returnvalue_location _returnvalue_rotation (0.01 0.01 0.01)) 0.02) false false))))

(fn `Upgrade`
  (params (Level :type Integer))
  (locals (Deleted :type Boolean))
  (set `self.CurrentLevel` Level)
  (`self.SetVisibility`)
  (set `/Game/Blueprints/VRGameMode.PowerStationLevel` (`self.CurrentLevel`) (`self.VRGameMode`))
  (`self.SetVariables`))

(fn `UserConstructionScript`)