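; Upgradeable storage building in a VR game that absorbs overlapping nuclear waste actors while below capacity and reports its totals to VRGameMode.
; Capacity comes from DT_BuildingInfo by level, scaled by the game mode's upgrade multiplier.
; Name-filtered events drive hover, selection, upgrades and demolition, with per-level mesh roots toggled for display and ghost previews.
; Tick updates selection and the player-facing capacity widget; demolition spawns an empty plot and respawns stored waste.
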(event `/Game/Blueprints/Interface/I_Storage.StorageUpgrade`
  (`self.SetValues`))

(event `/Game/Blueprints/Interface/I_Storage.GetStorage`
  (bind _vrgamemode (`self.VRGameMode`))
  (bind _vrgamemode_2 (`self.VRGameMode`))
  (set `/Game/Blueprints/VRGameMode.StorageMax` (+ (`/Game/Blueprints/VRGameMode.StorageMax` _vrgamemode) (`self.MaxStorage`)) _vrgamemode)
  (set `/Game/Blueprints/VRGameMode.WasteStored` (+ (`/Game/Blueprints/VRGameMode.WasteStored` _vrgamemode_2) (`self.CurrentStorage`)) _vrgamemode_2))

(event `/Game/Blueprints/Interface/I_UpgradeAble.GhostVisiblity`
  (params (Level :type Integer))
  (`self.GhostVisibility` Level))

(event `/Game/Blueprints/Interface/I_InteractivePlot.SelectOff`
  (params (Name :type String))
  (if (`KismetStringLibrary.EqualEqual_StrStr` Name (`KismetSystemLibrary.GetObjectName` self))
    (set `self.Selected` false)))

(event `/Game/Blueprints/Interface/I_InteractivePlot.SelectOn`
  (params (Name :type String))
  (if (`KismetStringLibrary.EqualEqual_StrStr` Name (`KismetSystemLibrary.GetObjectName` self))
    (set `self.Selected` true)))

(event `/Game/Blueprints/Interface/I_InteractivePlot.HoverOn`
  (params (Name :type String))
  (if (`KismetStringLibrary.EqualEqual_StrStr` Name (`KismetSystemLibrary.GetObjectName` self))
    (set `self.Hovered` true)
    (set `self.CurrentSelectionCounter` (`self.SelectionCounter`))))

(event `self.ReceiveBeginPlay`
  (`SceneComponent.SetVisibility` (`self.UpgradeLevel0`) false false)
  (`SceneComponent.SetVisibility` (`self.UpgradeLevel1`) false false)
  (`SceneComponent.SetVisibility` (`self.UpgradeLevel2`) false false)
  (`SceneComponent.SetVisibility` (`self.UpgradeLevel3`) false false)
  (`KismetSystemLibrary.Delay` 0.05)
  (`SceneComponent.SetVisibility` (`self.SelectedBox`) (`self.Hovered`) true)
  (`KismetArrayLibrary.Array_Add` (`self.UpgradeLevelsRoots`) (`self.UpgradeLevel0`))
  (`KismetArrayLibrary.Array_Add` (`self.UpgradeLevelsRoots`) (`self.UpgradeLevel1`))
  (`KismetArrayLibrary.Array_Add` (`self.UpgradeLevelsRoots`) (`self.UpgradeLevel2`))
  (`KismetArrayLibrary.Array_Add` (`self.UpgradeLevelsRoots`) (`self.UpgradeLevel3`))
  (`self.SetVisibility`)
  (bind _asvrgame_mode (cast `/Game/Blueprints/VRGameMode` (`GameplayStatics.GetGameMode`)))
  (bind _output_get (set `self.VRGameMode` _asvrgame_mode))
  (`KismetArrayLibrary.Array_Add` (`/Game/Blueprints/VRGameMode.AllBuildings` _output_get) (`KismetStringLibrary.Conv_StringToName` (`KismetStringLibrary.Concat_StrStr` "Storage" (`KismetStringLibrary.Conv_IntToString` (`self.CurrentLevel`)))))
  (`self.SetValues`)
  (bind _asvrpawn (cast `/Game/Blueprints/VRPawn` (`GameplayStatics.GetPlayerPawn` 0)))
  (add `/Game/Blueprints/VRPawn.StorageVisible` _asvrpawn (delegate `SetWidgetVis`)))

(event `/Game/Blueprints/Interface/I_Demolishable.IDemolish`
  (params (IName :type String))
  (if (`KismetStringLibrary.EqualEqual_StrStr` IName (`KismetSystemLibrary.GetObjectName` self))
    (`self.Demolish`)))

(event `SetWidgetVis`
  (params (IsVisible :type Boolean))
  (`SceneComponent.SetVisibility` (`self.StorageWidget`) IsVisible false))

(event `/Game/Blueprints/Interface/I_UpgradeAble.IUpgrade`
  (params (Name :type String) (UpgradeLevel :type Integer))
  (if (`KismetStringLibrary.EqualEqual_StrStr` Name (`KismetSystemLibrary.GetObjectName` self))
    (`self.Upgrade` UpgradeLevel)
    (`self.SetValues`)))

(event `/Game/Blueprints/Interface/I_InteractivePlot.GetInteractiveValues`
  (bind _asvrpawn (cast `/Game/Blueprints/VRPawn` (`GameplayStatics.GetPlayerPawn` 0)))
  (`/Game/Blueprints/Interface/I_InteractivePlot.SendInteractiveValues` _asvrpawn "Storage" (`self.CurrentLevel`)))

(event `self.ReceiveTick`
  (params (DeltaSeconds :type "Float (single-precision)"))
  (bind _selected (`self.Selected`))
  (bind _returnvalue (or (`self.Hovered`) _selected))
  (`|ExecutionSequence`
    (:`then_0`
      (if (!= _returnvalue (`SceneComponent.IsVisible` (`self.SelectedBox`)))
        (`SceneComponent.SetVisibility` (`self.SelectedBox`) _returnvalue true)
        (if (not _selected)
          (`self.SetVisibility`)))
      (if (and (`self.Hovered`) (> (`self.CurrentSelectionCounter`) 0.0))
        (set `self.CurrentSelectionCounter` (- (`self.CurrentSelectionCounter`) (`GameplayStatics.GetWorldDeltaSeconds`)))
        (elif (not (`self.Selected`))
          (set `self.Hovered` false))))
    (:`then_1`
      ;[1 1 1] Widget Lookat player
      (bind _asvrpawn (cast `/Game/Blueprints/VRPawn` (`GameplayStatics.GetPlayerPawn` 0)))
      (`SceneComponent.K2_SetWorldRotation` (`self.StorageWidget`) (`KismetMathLibrary.FindLookAtRotation` (`SceneComponent.K2_GetComponentLocation` (`self.StorageWidget`)) (`SceneComponent.K2_GetComponentLocation` (`/Game/Blueprints/VRPawn.Camera` _asvrpawn))) false false)
      ;[1 1 1] Set Widget varibles
      (`KismetSystemLibrary.Delay` 0.2)
      (bind _asw_storage_cap (cast `/Game/Blueprints/Widgets/W_StorageCap` (`WidgetComponent.GetUserWidgetObject` (`self.StorageWidget`))))
      (set `/Game/Blueprints/Widgets/W_StorageCap.fCurrentStorage` (`self.CurrentStorage`) _asw_storage_cap)
      (set `/Game/Blueprints/Widgets/W_StorageCap.fMaxStorage` (`self.MaxStorage`) _asw_storage_cap))))

(event `self.Box.OnComponentBeginOverlap`
  (params (OverlappedComponent :type "PrimitiveComponent Object Reference") (OtherActor :type "Actor Object Reference") (OtherComp :type "PrimitiveComponent Object Reference") (OtherBodyIndex :type Integer) (bFromSweep :type Boolean) (SweepResult :type "HitResult Structure (by ref)"))
  (bind _asbp_nuclear_waste (cast `/Game/Blueprints/Actors/PickupObjects/BP_NuclearWaste` OtherActor))
  (if (> (`self.MaxStorage`) (`self.CurrentStorage`))
    (set `self.CurrentStorage` (+ (`/Game/Blueprints/Actors/PickupObjects/BP_NuclearWaste.WasteCarried` _asbp_nuclear_waste) (`self.CurrentStorage`)))
    (`self.K2_DestroyActor` _asbp_nuclear_waste)))

(fn `Demolish`
  (locals (Deleted :type Boolean))
  (bind (_returnvalue_x _returnvalue_y) (`KismetMathLibrary.BreakVector` (`SceneComponent.K2_GetComponentLocation` (`self.DefaultSceneRoot`))))
  (for (_array_element _array_index) (`/Game/Blueprints/VRGameMode.AllBuildings` (`self.VRGameMode`))
    (if (and (not (`local.Deleted`)) (== _array_element (`KismetStringLibrary.Conv_StringToName` (`KismetStringLibrary.Concat_StrStr` "Storage" (`KismetStringLibrary.Conv_IntToString` (`self.CurrentLevel`))))))
      (`KismetArrayLibrary.Array_Remove` (`/Game/Blueprints/VRGameMode.AllBuildings` (`self.VRGameMode`)) _array_index)
      (set `local.Deleted` false)))
  (`|SpawnActorFromClass` "/Game/Blueprints/Actors/Buildings/BP_EmptyPlot.BP_EmptyPlot_C" (`SceneComponent.K2_GetComponentToWorld` (`self.DefaultSceneRoot`)) "Undefined" "OverrideRootScale" null null)
  (for _ (range (+ (`KismetMathLibrary.Round` (/ (`self.CurrentStorage`) 20.0)) 1))
    (if (> (- (`self.CurrentStorage`) 20.0) 0.0)
      (bind _returnvalue (`|SpawnActorFromClass` "/Game/Blueprints/Actors/PickupObjects/BP_NuclearWaste.BP_NuclearWaste_C" (`KismetMathLibrary.MakeTransform` (`KismetMathLibrary.MakeVector` _returnvalue_x _returnvalue_y 400.0) (struct) (0.2 0.2 0.2)) "Undefined" "OverrideRootScale" null null))
      (bind _output_get (set `/Game/Blueprints/Actors/PickupObjects/BP_NuclearWaste.WasteCarried` 20.0 _returnvalue))
      (set `self.CurrentStorage` (- (`self.CurrentStorage`) _output_get))
      (else
        (bind _returnvalue_2 (`|SpawnActorFromClass` "/Game/Blueprints/Actors/PickupObjects/BP_NuclearWaste.BP_NuclearWaste_C" (`KismetMathLibrary.MakeTransform` (`KismetMathLibrary.MakeVector` _returnvalue_x _returnvalue_y 400.0) (struct) (0.2 0.2 0.2)) "Undefined" "OverrideRootScale" null null))
        (bind _output_get_2 (set `/Game/Blueprints/Actors/PickupObjects/BP_NuclearWaste.WasteCarried` (`self.CurrentStorage`) _returnvalue_2))
        (set `self.CurrentStorage` (- (`self.CurrentStorage`) _output_get_2)))))
  (`self.K2_DestroyActor`))

(fn `GhostVisibility`
  (params (Level :type Integer))
  (locals (LocBuildingID :type Integer))
  (for (_ _array_index) (`self.UpgradeLevelsRoots`)
    (`SceneComponent.SetVisibility` (`|GetArrayItem` (`self.UpgradeLevelsRoots`) _array_index) (== _array_index Level) true)))

(fn `SetValues`
  (bind _returnvalue (`|GetDataTableRow` "/Game/Blueprints/DataManagement/DT_BuildingInfo.DT_BuildingInfo" (`KismetStringLibrary.Conv_StringToName` (`KismetStringLibrary.Concat_StrStr` "Storage" (`KismetStringLibrary.Conv_IntToString` (`self.CurrentLevel`)))))
    (:`then`
      (set `self.MaxStorage` (* (`.StorageProvided_23_271D7A054F000141D64995B882ECA2F9` (break `/Game/Blueprints/DataManagement/Struct_Buildings` _returnvalue)) (`/Game/Blueprints/VRGameMode.UpStorageMulti` (`self.VRGameMode`)))))))

(fn `SetVisibility`
  (locals (LocBuildingID :type Integer))
  (for (_ _array_index) (`self.UpgradeLevelsRoots`)
    (`SceneComponent.SetVisibility` (`|GetArrayItem` (`self.UpgradeLevelsRoots`) _array_index) (== _array_index (`self.CurrentLevel`)) true)))

(fn `Upgrade`
  (params (Level :type Integer))
  (locals (Deleted :type Boolean))
  (bind _allbuildings (`/Game/Blueprints/VRGameMode.AllBuildings` (`self.VRGameMode`)))
  (set `self.CurrentLevel` Level)
  (`self.SetVisibility`)
  (for (_array_element _array_index) _allbuildings
    (if (and (not (`local.Deleted`)) (== _array_element (`KismetStringLibrary.Conv_StringToName` (`KismetStringLibrary.Concat_StrStr` "Storage" (`KismetStringLibrary.Conv_IntToString` (- (`self.CurrentLevel`) 1))))))
      (`KismetArrayLibrary.Array_Remove` (`/Game/Blueprints/VRGameMode.AllBuildings` (`self.VRGameMode`)) _array_index)
      (set `local.Deleted` true)))
  (`KismetArrayLibrary.Array_Add` _allbuildings (`KismetStringLibrary.Conv_StringToName` (`KismetStringLibrary.Concat_StrStr` "Storage" (`KismetStringLibrary.Conv_IntToString` (`self.CurrentLevel`))))))

(fn `UserConstructionScript`)