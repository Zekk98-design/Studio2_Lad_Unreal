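; BP_Blockade is a selectable building actor that keeps a set of level objects hidden until it is unlocked.
; On BeginPlay it hides ObjectsToUnlock and sets Price from the number implementing I_EmptyPlot; UnlockBlockade reveals them and destroys the blockade.
; Name-matched hover and select events drive SelectBox visibility in Tick, with a countdown that expires hover.
; It reports itself as "Blockade" to the VRPawn through GetInteractiveValues.
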(event `self.SelectOff`
  (params (Name :type String))
  (if (`KismetStringLibrary.EqualEqual_StrStr` Name (`KismetSystemLibrary.GetObjectName` self))
    (set `self.Selected` false)))

(event `self.ReceiveBeginPlay`
  (for _array_element (`self.ObjectsToUnlock`)
    (`/Engine/EditorBlueprintResources/StandardMacros.IsValid` _array_element
      (:`Is Valid`
        (`self.SetActorHiddenInGame` _array_element true)
        (if (`KismetSystemLibrary.DoesImplementInterface` _array_element "/Game/Blueprints/Interface/I_EmptyPlot.I_EmptyPlot_C")
          (`/Engine/EditorBlueprintResources/StandardMacros.IncrementInt` (`self.NumberOfPlots`))))))
  (set `self.Price` (* (`self.NumberOfPlots`) 100.0)))

(event `self.SelectOn`
  (params (Name :type String))
  (if (`KismetStringLibrary.EqualEqual_StrStr` Name (`KismetSystemLibrary.GetObjectName` self))
    (set `self.Selected` true)))

(event `self.HoverOn`
  (params (Name :type String))
  (if (`KismetStringLibrary.EqualEqual_StrStr` Name (`KismetSystemLibrary.GetObjectName` self))
    (set `self.Hovered` true)
    (set `self.CurrentSelectionCounter` (`self.SelectionCounter`))))

(event `/Game/Blueprints/Interface/I_Blockade.UnlockBlockade`
  (params (Name :type String))
  (for _array_element (`self.ObjectsToUnlock`)
    (`/Engine/EditorBlueprintResources/StandardMacros.IsValid` _array_element
      (:`Is Valid`
        (`self.SetActorHiddenInGame` _array_element false)
        (`self.K2_DestroyActor`)))))

(event `self.GetInteractiveValues`
  (bind _asvrpawn (cast `/Game/Blueprints/VRPawn` (`GameplayStatics.GetPlayerPawn` 0)))
  (`self.SendInteractiveValues` _asvrpawn "Blockade" 0))

(event `self.ReceiveTick`
  (params (DeltaSeconds :type "Float (single-precision)"))
  (bind _returnvalue (or (`self.Hovered`) (`self.Selected`)))
  (if (!= _returnvalue (`SceneComponent.IsVisible` (`self.SelectBox`)))
    (`SceneComponent.SetVisibility` (`self.SelectBox`) _returnvalue true))
  (if (and (`self.Hovered`) (> (`self.CurrentSelectionCounter`) 0.0))
    (set `self.CurrentSelectionCounter` (- (`self.CurrentSelectionCounter`) (`GameplayStatics.GetWorldDeltaSeconds`)))
    (elif (not (`self.Selected`))
      (set `self.Hovered` false))))

(fn `UserConstructionScript`)