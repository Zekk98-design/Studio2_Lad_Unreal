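; BP_Clouds is a moving emitter that scatters BP_Cloud actors along its path.
; Every Tick shifts the actor 10 units along world X from its Billboard component's location, so speed depends on frame rate.
; A Delay on Tick throttles spawning to roughly five clouds per second, each at one-tenth scale, randomly offset within 500 units on each axis around the Billboard.
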(event `self.ReceiveBeginPlay`)

(event `self.ReceiveTick`
  (params (DeltaSeconds :type "Float (single-precision)"))
  (bind (_returnvalue_x _returnvalue_y _returnvalue_z) (`KismetMathLibrary.BreakVector` (`SceneComponent.K2_GetComponentLocation` (`self.Billboard`))))
  (`self.K2_SetActorLocation` self (`KismetMathLibrary.MakeVector` (+ _returnvalue_x 10.0) _returnvalue_y _returnvalue_z) false false)
  (`KismetSystemLibrary.Delay` 0.2)
  (`|SpawnActorFromClass` "/Game/Blueprints/Paticals/BP_Cloud.BP_Cloud_C" (`KismetMathLibrary.MakeTransform` (`KismetMathLibrary.MakeVector` (+ (.x (.location (`SceneComponent.K2_GetComponentToWorld` (`self.Billboard`)))) (`KismetMathLibrary.RandomFloatInRange` -500.0 500.0)) (+ (.y (.location (`SceneComponent.K2_GetComponentToWorld` (`self.Billboard`)))) (`KismetMathLibrary.RandomFloatInRange` -500.0 500.0)) (+ (.z (.location (`SceneComponent.K2_GetComponentToWorld` (`self.Billboard`)))) (`KismetMathLibrary.RandomFloatInRange` -500.0 500.0))) (.rotation (`SceneComponent.K2_GetComponentToWorld` (`self.Billboard`))) (0.1 0.1 0.1)) "Undefined" "OverrideRootScale" null null))

(fn `UserConstructionScript`)