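; Game mode for a VR nuclear-powered settlement management sim, calling YouWin on the player pawn once the days to survive run out.
; A Delay-throttled Tick rebuilds totals from power plant and building data tables, then updates interdependent money, population, waste, research, radiation, power, storage, health and happiness.
; Per-day rates are scaled by day speed and call interval.
; Random data-table events go to an interface widget, and choices adjust stats by name.
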(event `self.ReceiveBeginPlay`
  (`KismetSystemLibrary.Delay` 0.2)
  (bind _asvrpawn (cast `/Game/Blueprints/VRPawn` (`GameplayStatics.GetPlayerPawn` 0)))
  (set `self.PlayerPawn` _asvrpawn))

(event `self.ReceiveTick`
  (params (DeltaSeconds :type "Float (single-precision)"))
  (bind _returnvalue (- (* (`self.DaysToSurvive`) 24.0) (`self.TimePast`)))
  (set `self.TimeLeft` _returnvalue)
  (if (< _returnvalue 0.0)
    (`self.EndGame`)
    (else
      (`KismetSystemLibrary.Delay` (`self.CallDelay`))
      (`|ExecutionSequence`
        (:`then_0`
          (bind _returnvalue_2 (`|GetDataTableRow` "/Game/Blueprints/DataManagement/DT_Powerplant.DT_Powerplant" (`KismetStringLibrary.Conv_StringToName` (`KismetStringLibrary.Concat_StrStr` "Powerplant" (`KismetStringLibrary.Conv_IntToString` (`self.PowerStationLevel`)))))
            (:`then`
              (bind (_maxpower _wasteproduced) (break `/Game/Blueprints/DataManagement/Struct_Powerplant` _returnvalue_2))
              (set `self.MaxPower` _maxpower)
              (set `self.WasteProduced` _wasteproduced)
              (set `self.PopulationCap` 0.0)
              (set `self.PowerRequired` 0.0)
              (set `self.StorageBuildingBonus` 0.0)
              (set `self.PopulationHealthBuildings` 0.0)
              (set `self.HappinessBuildingBonus` 0.0)
              (set `self.MoneyBuildings` 0.0)
              (set `self.ResearchBuildingBonus` 0.0)
              (set `self.PowerBuildingsBonus` 0.0)
              (set `self.RadiationBuildingsReduction` 0.0)
              (set `self.RadiationLevel0` 0.0)
              (set `self.RadiationLevel1` 0.0)
              (set `self.RadiationLevel2` 0.0)
              (set `self.RadiationLevel3` 0.0)
              (`self.SetValues`))))
        (:`then_1`
          (`self.SetMoney`)
          (`self.SetPopulation`)
          (`self.SetNuclearWaste`)
          (`self.SetResearch`)
          (`self.SetRadition`)
          (`self.SetPower`)
          (`self.SetStorage`)
          (`self.SetPopulationHealth`)
          (`self.SetHappiness`))))))

(event `/Game/Blueprints/Interface/EventSystem.GetOptionChosen`
  (params (Option1Chosen :type Boolean))
  (bind _returnvalue (`|GetDataTableRow` "/Game/Blueprints/DataManagement/DT_RandomEvents.DT_RandomEvents" (`self.CurrentEventName`))
    (:`then`
      (if Option1Chosen
        (bind (_eventname _description _option1text _option1variable1isgood _option1variable1name _option1variable1value _option1variable2isgood _option1variable2name _option1variable2value _option2text _option2variable1isgood _option2variable1name _option2variable1value _option2variable2isgood _option2variable2name _option2variable2value) (break `/Game/Blueprints/DataManagement/Struct_RandomEvents` _returnvalue))
        (`self.ApplyEvent` _option1variable1name _option1variable1value)
        (`self.ApplyEvent` _option1variable2name _option1variable2value)
        (`self.ApplyEvent` _option2variable1name _option2variable1value)
        (`self.ApplyEvent` _option2variable2name _option2variable2value)))))

(fn `ApplyEvent`
  (params (ValueName :type String) (ValueAmount :type "Float (double-precision)"))
  (switch `string` ValueName
    (:`Money`
      (set `self.Money` (+ ValueAmount (`self.Money`))))
    (:`Population`
      (set `self.Population` (+ ValueAmount (`self.Population`))))
    (:`NuclearWaste`
      (set `self.NuclearWaste` (+ ValueAmount (`self.NuclearWaste`))))
    (:`Research`
      (set `self.Research` (+ ValueAmount (`self.Research`))))
    (:`Happiness`
      (set `self.Happiness` (+ ValueAmount (`self.Happiness`))))
    (:`Radiation`
      (set `self.Radiation` (+ ValueAmount (`self.Radiation`))))
    (:`PopulationHealth`
      (set `self.PopulationHealth` (+ ValueAmount (`self.PopulationHealth`))))))

(fn `EndGame`
  (`/Game/Blueprints/Interface/I_Player.YouWin` (`self.PlayerPawn`)))

(fn `RandomEvent`
  (bind _outrownames (`DataTableFunctionLibrary.GetDataTableRowNames` "/Game/Blueprints/DataManagement/DT_RandomEvents.DT_RandomEvents"))
  (bind _foundwidgets (`WidgetBlueprintLibrary.GetAllWidgetsWithInterface` "/Game/Blueprints/Interface/EventSystem.EventSystem_C"))
  (bind _output (`|GetArrayItem` _outrownames (`KismetMathLibrary.RandomIntegerInRange` 0 (- (`KismetArrayLibrary.Array_Length` _outrownames) 1))))
  (set `self.CurrentEventName` _output)
  (message `/Game/Blueprints/Interface/EventSystem.SetWidgetEvents` (`|GetArrayItem` _foundwidgets) _output))

(fn `SetHappiness`
  (locals (HappinessPerDay :type "Float (double-precision)"))
  (bind _returnvalue (`KismetMathLibrary.FClamp` (/ (`self.CurrentPower`) (`self.PowerRequired`)) 0.25 1.25))
  (set `local.HappinessPerDay` (+ (* (- (+ _returnvalue (* _returnvalue (`self.HappinessBuildingBonus`))) 1.0) (`self.HappinessModifier`)) (* (`self.PopulationHealth`) 0.5)))
  (set `self.Happiness` (`KismetMathLibrary.FClamp` (+ (/ (`local.HappinessPerDay`) (/ (`self.DaySpeed`) (`self.CallDelay`))) (`self.Happiness`)) 0.1 (`self.PopulationHealth`))))

(fn `SetMoney`
  (locals (MoneyPerDay :type "Float (double-precision)"))
  (set `local.MoneyPerDay` (* (+ (* (`self.Happiness`) (`self.Population`)) (`self.MoneyBuildings`) (`self.MoneyIncomeBase`)) (`self.MoneyMultiplier`)))
  (set `self.Money` (+ (/ (`local.MoneyPerDay`) (/ (`self.DaySpeed`) (`self.CallDelay`))) (`self.Money`))))

(fn `SetNuclearWaste`
  (locals (NuclearWastePerDay :type "Float (double-precision)"))
  (set `local.NuclearWastePerDay` (* (`self.CurrentPower`) (`self.WasteProduced`) (`self.NuclearWasteMulitplier`)))
  (set `self.NuclearWaste` (+ (/ (`local.NuclearWastePerDay`) (/ (`self.DaySpeed`) (`self.CallDelay`))) (`self.NuclearWaste`))))

(fn `SetPopulation`
  (locals (PopulationPerDay :type "Float (double-precision)"))
  (bind _output_get (set `local.PopulationPerDay` (* (`self.PopulationMultiplier`) (+ (- (+ (`self.Happiness`) 0.5) 1.0) (- 1.0 (/ (`self.Population`) (`self.PopulationCap`)))))))
  (`KismetSystemLibrary.PrintString` (`KismetStringLibrary.Conv_DoubleToString` _output_get))
  (set `self.Population` (`KismetMathLibrary.FClamp` (+ (/ (`local.PopulationPerDay`) (/ (`self.DaySpeed`) (`self.CallDelay`))) (`self.Population`)) 1.0 (`self.PopulationCap`))))

(fn `SetPopulationHealth`
  (set `self.PopulationHealth` (`KismetMathLibrary.FClamp` (/ (- (`self.Population`) (/ (`self.Radiation`) (+ (`self.PopulationHealthRadiationPerPerson`) (`self.PopulationHealthBuildings`)))) (`self.Population`)))))

(fn `SetPower`
  (set `self.PowerRequired` (+ (`self.PowerRequired`) (* (`self.Population`) (`self.PowerMultiplier`)))))

(fn `SetRadition`
  (set `self.Radiation` (* (- (`self.NuclearWaste`) (+ (* (`self.RadiationLevel0`) 0.7) (* (`self.RadiationLevel1`) 0.8) (* (`self.RadiationLevel2`) 0.9) (* (`self.RadiationLevel3`) 1.0) (`self.RadiationBuildingsReduction`) (- (`self.StorageMax`) (`self.NuclearWaste`)))) (`self.RadiationModifier`))))

(fn `SetResearch`
  (locals (ResearchPerDay :type "Float (double-precision)"))
  (set `local.ResearchPerDay` (+ (`self.ResearchBase`) (* (`self.ResearchBuildingBonus`) (`self.ResearchMultiplier`))))
  (set `self.Research` (+ (/ (`local.ResearchPerDay`) (/ (`self.DaySpeed`) (`self.CallDelay`))) (`self.Research`))))

(fn `SetStorage`
  (set `self.StorageMax` (+ (`self.StorageBuildingBonus`) (`self.BaseStorage`))))

(fn `SetValues`
  (for _array_element (`self.AllBuildings`)
    (bind _returnvalue (`|GetDataTableRow` "/Game/Blueprints/DataManagement/DT_BuildingInfo.DT_BuildingInfo" _array_element)
      (:`then`
        (bind (_id _active _price _name _level _moneyprovided _powerrequired _populationprovided _researchprovided _storageprovided _happinessprovided _radiationreduction _populationhealth) (break `/Game/Blueprints/DataManagement/Struct_Buildings` _returnvalue))
        (set `self.MoneyBuildings` (+ _moneyprovided (`self.MoneyBuildings`)))
        (set `self.PowerRequired` (+ _powerrequired (`self.PowerRequired`)))
        (set `self.PopulationCap` (+ _populationprovided (`self.PopulationCap`)))
        (set `self.ResearchBuildingBonus` (+ _researchprovided (`self.ResearchBuildingBonus`)))
        (set `self.HappinessBuildingBonus` (+ _happinessprovided (`self.HappinessBuildingBonus`)))
        (set `self.RadiationBuildingsReduction` (+ _radiationreduction (`self.RadiationBuildingsReduction`)))
        (set `self.PopulationHealthBuildings` (+ _populationhealth (`self.PopulationHealthBuildings`)))
        (set `self.StorageBuildingBonus` (+ _storageprovided (`self.StorageBuildingBonus`)))
        (switch `int` _level
          (:`0`
            (set `self.RadiationLevel0` (+ _storageprovided (`self.RadiationLevel0`))))
          (:`1`
            (set `self.RadiationLevel1` (+ _storageprovided (`self.RadiationLevel1`))))
          (:`2`
            (set `self.RadiationLevel2` (+ _storageprovided (`self.RadiationLevel2`))))
          (:`3`
            (set `self.RadiationLevel3` (+ _storageprovided (`self.RadiationLevel3`))))))
      (:`RowNotFound`
        (`KismetSystemLibrary.PrintString` "-------- Data Table Row Not Found --------"))))
  (return))

(fn `UserConstructionScript`)